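; BP_SceneTransition is an overlap trigger that moves the player to another level.
; In the Atrium, it first stores its SpawnPosition in GI_StoreInformation as the Atrium spawn location.
; It then clears the character's RoomLoaded flag, sets the game instance's anxiety density from AnxietyNextLevel and starts breathing music.
; A camera fade and short delay precede opening the referenced level.
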(event `self.ReceiveBeginPlay`
  (bind _asgi_store_information (cast `/Game/StopAndBreathe/Blueprints/GI_StoreInformation` (`GameplayStatics.GetGameInstance`)))
  (set `self.gameInstance` _asgi_store_information))

(event `self.ReceiveActorBeginOverlap`
  (params (OtherActor :type "Actor Object Reference"))
  (bind _asbp_third_person_character (cast `/Game/ThirdPerson/Blueprints/BP_ThirdPersonCharacter` OtherActor))
  ;[0.4161 1 0.2142] If the player was in the Atrium, remember the door they entered from and store it
  (bind _returnvalue (`GameplayStatics.GetCurrentLevelName` true))
  (if (`KismetStringLibrary.EqualEqual_StrStr` _returnvalue "LEVEL0_Atrium")
    (bind _asgi_store_information (cast `/Game/StopAndBreathe/Blueprints/GI_StoreInformation` (`GameplayStatics.GetGameInstance`)))
    (set `/Game/StopAndBreathe/Blueprints/GI_StoreInformation.atriumSpawnLocation` (`SceneComponent.K2_GetComponentLocation` (`self.SpawnPosition`)) _asgi_store_information))
  (set `/Game/ThirdPerson/Blueprints/BP_ThirdPersonCharacter.roomLoaded` false _asbp_third_person_character)
  (if (`self.anxietyNextLevel?`)
    (set `/Game/StopAndBreathe/Blueprints/GI_StoreInformation.anxietyDensityValue` 0.0 (`self.gameInstance`))
    (else
      (set `/Game/StopAndBreathe/Blueprints/GI_StoreInformation.anxietyDensityValue` 1.0 (`self.gameInstance`))))
  (`/Game/StopAndBreathe/Blueprints/GI_StoreInformation.PlayBreathingMusic` (`self.gameInstance`))
  ;[0.8482 0.5565 1] Load the next level
  (`PlayerCameraManager.StartCameraFade` :`self` (`GameplayStatics.GetPlayerCameraManager` 0) :`ToAlpha` 1.0 :`Duration` 2.0 :`bHoldWhenFinished` true)
  (`KismetSystemLibrary.Delay` 2.5)
  (`GameplayStatics.OpenLevelBySoftObjectPtr` (`self.Level`)))

(fn `UserConstructionScript`)