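; BP_RotatingPlatform is a platform that rotates in steps in response to breath states, one direction on Inhale and the other on Exhale.
; ObjectFunction passes the direction to RotatePlatform, which sets a target clamped between min and max, using a step size computed at BeginPlay.
; Tick advances a timer and lerps the Platform component's relative rotation on the enabled X, Y or Z axes, then commits the new angle.
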(event `self.ReceiveBeginPlay`
  ;[0.6022 0.7073 1] Calculate the rotation step angle from min, max, and # of steps
  (set `self.rotationStepValue` (/ (- (`self.maxRotationValue`) (`self.minRotationValue`)) (`self.rotationSteps`))))

(event `Rotate Platform`
  (params (Direction :type Integer :default 1))
  (bind _currentrotationvalue (`self.currentRotationValue`))
  ;[1 0.1982 0.8249] Rotate the Platform, if the Platform is Not Already Rotating
  (if (not (`self.rotating`))
    (set `self.newRotationValue` (`KismetMathLibrary.FClamp` (+ (* Direction (`self.rotationStepValue`)) (`self.currentRotationValue`)) (`self.minRotationValue`) (`self.maxRotationValue`)))
    (set `self.rotationTimer` 0.0)
    (if (not (or (== _currentrotationvalue (`self.minRotationValue`)) (== _currentrotationvalue (`self.maxRotationValue`))))
      (set `self.rotating` true))))

(event `self.ReceiveTick`
  (params (DeltaSeconds :type "Float (single-precision)"))
  (bind _returnvalue (`KismetMathLibrary.Lerp` (`self.currentRotationValue`) (`self.newRotationValue`) (/ (`self.rotationTimer`) (`self.rotationTime`))))
  ;[1 1 1] EventTick
  (`|ExecutionSequence`
    (:`then_0`
      ;;[1 0.9325 0.0737] Increment the rotation timer
      (if (< (`self.rotationTimer`) (`self.rotationTime`))
        (set `self.rotationTimer` (+ (`self.rotationTimer`) (`GameplayStatics.GetWorldDeltaSeconds`)))
        (else
          ;;;[1 0.03365 0.6143] Reset values
          (set `self.currentRotationValue` (`self.newRotationValue`))
          (set `self.rotating` false))))
    (:`then_1`
      ;;[0.1513 0.7556 1] Rotate the platform along the desire axis
      (`|ExecutionSequence`
        (:`then_0`
          (if (`self.RotateAlongX`)
            (set `self.X` _returnvalue)
            (`SceneComponent.K2_SetRelativeRotation` (`self.Platform`) (`KismetMathLibrary.MakeRotator` (`self.X`) (`self.Y`) (`self.Z`)) false false :!label _label)))
        (:`then_1`
          (if (`self.RotateAlongY`)
            (set `self.Y` _returnvalue)
            (goto _label)))
        (:`then_2`
          (if (`self.RotateAlongZ`)
            (set `self.Z` _returnvalue)
            (goto _label)))))))

(event `/Game/StopAndBreathe/Blueprints/Interactables/BPI_Interactable.ObjectFunction`
  (params (NewParam :type "/Game/StopAndBreathe/Blueprints/Interactables/ENUM_InteractableStates Enum" :default "NewEnumerator2"))
  (switch `/Game/StopAndBreathe/Blueprints/Interactables/ENUM_InteractableStates` NewParam
    (:`NewEnumerator0`
      (`self.Rotate Platform` 1))
    (:`NewEnumerator1`
      (`self.Rotate Platform` -1))))

(fn `UserConstructionScript`)