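; BP_SnapPoint is a placement marker that shows a box outline when a held BP_PickeableBox enters its snap radius.
; Every tick it queries SnapRadius for overlapping boxes and reveals BoxOutline if the first one is being held.
; The outline hides only once no boxes overlap, so releasing a box inside the radius leaves it visible.
; The graph handles this visual feedback only and does not move or snap the box.
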(event `self.ReceiveTick`
  (params (DeltaSeconds :type "Float (single-precision)"))
  (bind _overlappingactors (`PrimitiveComponent.GetOverlappingActors` (`self.SnapRadius`) "/Game/StopAndBreathe/Blueprints/Interactables/BP_PickeableBox.BP_PickeableBox_C"))
  (if (`KismetArrayLibrary.Array_IsNotEmpty` _overlappingactors)
    (bind _asbp_pickeable_box (cast `/Game/StopAndBreathe/Blueprints/Interactables/BP_PickeableBox` (`|GetArrayItem` _overlappingactors)))
    (if (`/Game/StopAndBreathe/Blueprints/Interactables/BP_PickeableBox.IsBeingHeld` _asbp_pickeable_box)
      (`SceneComponent.SetVisibility` (`self.BoxOutline`) true false))
    (else
      (`SceneComponent.SetVisibility` (`self.BoxOutline`) false false))))

(fn `UserConstructionScript`)