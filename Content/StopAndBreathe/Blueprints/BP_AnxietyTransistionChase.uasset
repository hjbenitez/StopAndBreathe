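; Trigger volume that blends anxiety screen effects as the player crosses it along the Y axis, apparently for a chase transition.
; On overlap, it sets start and end Y from the entry side, actor bounds and capsule radius, so intensity always rises toward +Y.
; While inside, Tick maps player position to lower FogOfWar material saturation and stronger post-process vignette.
; Leaving from either side stops updates and zeroes the GameInstance's anxiety density.
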(event `self.ReceiveActorEndOverlap`
  (params (OtherActor :type "Actor Object Reference"))
  (bind _asbp_third_person_character (cast `/Game/ThirdPerson/Blueprints/BP_ThirdPersonCharacter` OtherActor))
  (bind (_returnvalue_x _returnvalue_y) (`KismetMathLibrary.BreakVector` (`self.K2_GetActorLocation` _asbp_third_person_character)))
  (set `self.playerY` _returnvalue_y)
  (set `self.playerRadius` (`CapsuleComponent.GetScaledCapsuleRadius` (`Character.CapsuleComponent` _asbp_third_person_character)))
  (if (== (`KismetMathLibrary.SignOfFloat` (- (`self.playerY`) (`self.selfY`))) -1.0)
    (bind _asgi_store_information (cast `/Game/StopAndBreathe/Blueprints/GI_StoreInformation` (`GameplayStatics.GetGameInstance`)))
    (set `/Game/StopAndBreathe/Blueprints/GI_StoreInformation.anxietyDensityValue` 0.0 _asgi_store_information)
    (else
      (bind _asgi_store_information_2 (cast `/Game/StopAndBreathe/Blueprints/GI_StoreInformation` (`GameplayStatics.GetGameInstance`)))
      (set `/Game/StopAndBreathe/Blueprints/GI_StoreInformation.anxietyDensityValue` 0.0 _asgi_store_information_2)))
  (set `self.insideTrigger` false))

(event `self.ReceiveActorBeginOverlap`
  (params (OtherActor :type "Actor Object Reference"))
  (bind (_origin _boxextent) (`self.GetActorBounds` false))
  (bind (_origin_2 _boxextent_2) (`self.GetActorBounds` false))
  (bind _asbp_third_person_character (cast `/Game/ThirdPerson/Blueprints/BP_ThirdPersonCharacter` OtherActor))
  (bind (_returnvalue_x _returnvalue_y) (`KismetMathLibrary.BreakVector` (`self.K2_GetActorLocation` _asbp_third_person_character)))
  (set `self.playerY` _returnvalue_y)
  (set `self.playerRadius` (`CapsuleComponent.GetScaledCapsuleRadius` (`Character.CapsuleComponent` _asbp_third_person_character)))
  (if (== (`KismetMathLibrary.SignOfFloat` (- (`self.playerY`) (`self.selfY`))) -1.0)
    (set `self.startY` (`self.playerY`))
    (set `self.endY` (+ (.y _origin_2) (.y _boxextent_2) (`self.playerRadius`)))
    (else
      (set `self.endY` (`self.playerY`))
      (set `self.startY` (- (.y _origin) (.y _boxextent) (`self.playerRadius`)))))
  (set `self.insideTrigger` true))

(event `self.ReceiveBeginPlay`
  (bind (_returnvalue_x _returnvalue_y) (`KismetMathLibrary.BreakVector` (`self.K2_GetActorLocation`)))
  (bind _asbp_third_person_character (cast `/Game/ThirdPerson/Blueprints/BP_ThirdPersonCharacter` (`GameplayStatics.GetPlayerCharacter` 0)))
  (set `self.player` _asbp_third_person_character)
  (set `self.selfY` _returnvalue_y)
  (bind _asgi_store_information (cast `/Game/StopAndBreathe/Blueprints/GI_StoreInformation` (`GameplayStatics.GetGameInstance`)))
  (set `self.As GI Store Information` _asgi_store_information))

(event `self.ReceiveTick`
  (params (DeltaSeconds :type "Float (single-precision)"))
  (bind (_returnvalue_x _returnvalue_y) (`KismetMathLibrary.BreakVector` (`self.K2_GetActorLocation` (`self.player`))))
  (bind _fogofwar (`/Game/ThirdPerson/Blueprints/BP_ThirdPersonGameMode.fogOfWar` (`/Game/ThirdPerson/Blueprints/BP_ThirdPersonCharacter.gameMode` (`self.player`))))
  (bind ((`WeightedBlendables` _weightedblendables)) (break `PostProcessSettings` (`PostProcessVolume.Settings` (`/Game/ThirdPerson/Blueprints/BP_ThirdPersonCharacter.postProcessVolume` (`self.player`)))))
  (if (`self.insideTrigger`)
    (bind _output_get (set `self.temp` (/ (- _returnvalue_y (`self.startY`)) (- (`self.endY`) (`self.startY`)))))
    (`MaterialInstanceDynamic.SetScalarParameterValue` _fogofwar "saturationValue" (- 1.0 _output_get))
    (`KismetArrayLibrary.Array_Set` (`.Array` (break `WeightedBlendables` _weightedblendables)) 2 (make `WeightedBlendable` 1.0 _fogofwar))
    (set `PostProcessVolume.Settings` (make `PostProcessSettings` :`VignetteIntensity` (* (`/Game/ThirdPerson/Blueprints/BP_ThirdPersonCharacter.vignetteMax` (`self.player`)) (`self.temp`)) :`WeightedBlendables` _weightedblendables) (`/Game/ThirdPerson/Blueprints/BP_ThirdPersonCharacter.postProcessVolume` (`self.player`)))))

(fn `UserConstructionScript`)