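; BP_Door is a two-panel door actor that opens and closes in response to interaction events.
; ActivateInteraction hides both panels by shrinking them to near-zero world scale rather than animating them, and CancelInteraction restores their original scales.
; The construction script gathers the two door components and caches those starting scales.
; Both events play the same open/close sound at the panels' midpoint inside the loop, so once per panel.
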(event `/Game/StopAndBreathe/Blueprints/Interfaces/BPI_Interactable.ActivateInteraction`
  (for _array_element (`self.DoorArray`)
    (`SceneComponent.SetWorldScale3D` _array_element (0.001 0.001 0.001))
    (`GameplayStatics.PlaySoundAtLocation` "/Game/Audio/MetaSounds/MS_DoorOpenClose.MS_DoorOpenClose" (`KismetMathLibrary.VLerp` (`SceneComponent.K2_GetComponentLocation` (`self.Door1`)) (`SceneComponent.K2_GetComponentLocation` (`self.Door`)) 0.5) (struct) 1.0 1.0 0.0 null null null null)))

(event `/Game/StopAndBreathe/Blueprints/Interfaces/BPI_Interactable.CancelInteraction`
  (for (_array_element _array_index) (`self.DoorArray`)
    (`SceneComponent.SetWorldScale3D` _array_element (`|GetArrayItem` (`self.DoorStartingScale`) _array_index))
    (`GameplayStatics.PlaySoundAtLocation` "/Game/Audio/MetaSounds/MS_DoorOpenClose.MS_DoorOpenClose" (`KismetMathLibrary.VLerp` (`SceneComponent.K2_GetComponentLocation` (`self.Door1`)) (`SceneComponent.K2_GetComponentLocation` (`self.Door`)) 0.5) (struct) 1.0 1.0 0.0 null null null null)))

(fn `UserConstructionScript`
  (bind _output_get (set `self.DoorArray` (`|MakeArray` (`self.Door`) (`self.Door1`))))
  (for _array_element _output_get
    (`KismetArrayLibrary.Array_Add` (`self.DoorStartingScale`) (`SceneComponent.K2_GetComponentScale` _array_element))))