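; Game instance that keeps player progress (level, stars, anxiety values, Atrium state) and music across levels.
; SaveData copies changed fields into a SaveGameOMIG object and writes its slot; LoadData reads them back, substituting Atrium anxiety for density in "_Hall" levels.
; Persistent, paused A/B phase tracks crossfade, fading out for breathing or separately spawned chase music.
; Init is empty; its slot-loading logic is disconnected, so the save object arrives through SetData.
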(event `self.ReceiveInit`)

(fn `FadeChaseMusic`
  (bind _chasemusic (`self.ChaseMusic`)
    (:`then`
      (`AudioComponent.FadeOut` _chasemusic 2.0 0.0 "Linear"))
    (:`else`)))

(fn `InitializeMusic`
  (`self.AphaseMusic`
    (:`then`)
    (:`else`
      (`self.BphaseMusic`
        (:`then`)
        (:`else`
          (`GameplayStatics.PrimeAllSoundsInSoundClass` "/Engine/EngineSounds/Music.Music")
          (bind _returnvalue (`GameplayStatics.CreateSound2D` "/Game/Audio/MetaSounds/Music/MS_APhaseMusic.MS_APhaseMusic" 0.8 1.0 50.0 null true false))
          (bind _output_get (set `self.AphaseMusic` _returnvalue))
          (`AudioComponent.SetPaused` _output_get true)
          (bind _returnvalue_2 (`GameplayStatics.CreateSound2D` "/Game/Audio/MetaSounds/Music/MS_BPhaseMusic.MS_BPhaseMusic" 1.0 1.0 (`self.BphaseMusicProgress`) null true false))
          (bind _output_get_2 (set `self.BphaseMusic` _returnvalue_2))
          (`AudioComponent.SetPaused` _output_get_2 true))))))

(fn `LoadData`
  (`|ExecutionSequence`
    (:`then_0`
      (set `self.atriumAnxietyValue` (`/Game/StopAndBreathe/Blueprints/SaveGameOMIG.atriumAnxietyValue` (`self.As Save Game OMIG`)))
      (set `self.anxietyDensityValue` (`/Game/StopAndBreathe/Blueprints/SaveGameOMIG.anxietyDensityValue` (`self.As Save Game OMIG`))))
    (:`then_1`
      (set `self.starsCollected` (`/Game/StopAndBreathe/Blueprints/SaveGameOMIG.StarsCollected` (`self.As Save Game OMIG`)))
      (set `self.atriumFirstTimeCompleted?` (`/Game/StopAndBreathe/Blueprints/SaveGameOMIG.atriumFirstTimeCompleted?` (`self.As Save Game OMIG`))))
    (:`then_2`
      (bind _output_get (set `self.currentLevel` (`/Game/StopAndBreathe/Blueprints/SaveGameOMIG.currentLevel` (`self.As Save Game OMIG`))))
      (if (`KismetStringLibrary.EqualEqual_StrStr` (`KismetStringLibrary.GetSubstring` _output_get 6 5) "_Hall ")
        (set `self.anxietyDensityValue` (`self.atriumAnxietyValue`))))
    (:`then_3`
      (set `self.atriumSpawnLocation` (`/Game/StopAndBreathe/Blueprints/SaveGameOMIG.atriumSpawnLocation` (`self.As Save Game OMIG`))))))

(fn `PlayAPhaseMusic`
  (bind _aphasemusicprogress (`self.AphaseMusicProgress`))
  (bind _aphasemusic (`self.AphaseMusic`))
  (`AudioComponent.SetPaused` (`self.AphaseMusic`) false)
  (`AudioComponent.FadeOut` (`self.BphaseMusic`) 2.0 0.0 "Linear")
  (`AudioParameterControllerInterface.SetFloatParameter` _aphasemusic "StartTime" _aphasemusicprogress)
  (`AudioComponent.FadeIn` _aphasemusic 5.0 1.2 _aphasemusicprogress "Linear")
  (set `self.A phaseMusicIsPlaying` true)
  (set `self.B phaseMusicIsPlaying` false))

(fn `PlayBPhaseMusic`
  (`AudioComponent.SetPaused` (`self.BphaseMusic`) false)
  (`AudioComponent.FadeOut` (`self.AphaseMusic`) 2.0 0.0 "Linear")
  (`AudioParameterControllerInterface.SetFloatParameter` (`self.BphaseMusic`) "StartTime" 0.0)
  (`AudioComponent.FadeIn` (`self.BphaseMusic`) 5.0 1.2 0.0 "Linear")
  (set `self.A phaseMusicIsPlaying` false)
  (set `self.B phaseMusicIsPlaying` true))

(fn `PlayBreathingMusic`
  (`AudioComponent.FadeOut` (`self.AphaseMusic`) 1.0 0.0 "Linear")
  (`AudioComponent.FadeOut` (`self.BphaseMusic`) 2.0 0.0 "Linear")
  (set `self.A phaseMusicIsPlaying` false)
  (set `self.B phaseMusicIsPlaying` false))

(fn `PlayChaseMusic`
  (`AudioComponent.FadeOut` (`self.AphaseMusic`) 1.0 0.0 "Linear")
  (`AudioComponent.FadeOut` (`self.BphaseMusic`) 2.0 0.0 "Linear")
  (bind _returnvalue (`GameplayStatics.SpawnSound2D` "/Game/Audio/MetaSounds/Music/MS_ChaseMusic.MS_ChaseMusic" 1.0 1.0 0.0 null))
  (set `self.ChaseMusic` _returnvalue)
  (set `self.A phaseMusicIsPlaying` false)
  (set `self.B phaseMusicIsPlaying` false))

(fn `ResetGameInstance`
  (`|ExecutionSequence`
    (:`then_0`
      (set `self.A phaseMusicIsPlaying` false)
      (set `self.B phaseMusicIsPlaying` false))
    (:`then_1`
      (set `self.As Save Game OMIG` null)
      (set `self.sceneChange` false)
      (set `self.atriumAnxietyValue` 0.0)
      (set `self.currentLevel` "")
      (set `self.starsCollected` 0)
      (set `self.atriumSpawnLocation` (0.0 0.0 0.0))
      (set `self.anxietyDensityValue` 0.0))
    (:`then_2`
      (set `self.cameraAlpha` 0.0)
      (set `self.atriumFirstTimeCompleted?` false)
      (set `self.AphaseMusicProgress` 0.0)
      (set `self.BphaseMusicProgress` 0.0))))

(fn `SaveData`
  (`|ExecutionSequence`
    (:`then_0`
      (if (not (`KismetStringLibrary.EqualEqual_StrStr` (`self.currentLevel`) (`/Game/StopAndBreathe/Blueprints/SaveGameOMIG.currentLevel` (`self.As Save Game OMIG`))))
        (set `/Game/StopAndBreathe/Blueprints/SaveGameOMIG.currentLevel` (`self.currentLevel`) (`self.As Save Game OMIG`))))
    (:`then_1`
      (if (not (== (`self.starsCollected`) (`/Game/StopAndBreathe/Blueprints/SaveGameOMIG.StarsCollected` (`self.As Save Game OMIG`))))
        (set `/Game/StopAndBreathe/Blueprints/SaveGameOMIG.StarsCollected` (`self.starsCollected`) (`self.As Save Game OMIG`))))
    (:`then_2`
      (if (not (`KismetMathLibrary.NearlyEqual_FloatFloat` (`self.atriumAnxietyValue`) (`/Game/StopAndBreathe/Blueprints/SaveGameOMIG.atriumAnxietyValue` (`self.As Save Game OMIG`)) 0.05))
        (set `/Game/StopAndBreathe/Blueprints/SaveGameOMIG.atriumAnxietyValue` (`self.atriumAnxietyValue`) (`self.As Save Game OMIG`))))
    (:`then_3`
      (if (not (`KismetMathLibrary.NearlyEqual_FloatFloat` (`self.anxietyDensityValue`) (`/Game/StopAndBreathe/Blueprints/SaveGameOMIG.anxietyDensityValue` (`self.As Save Game OMIG`)) 0.05))
        (set `/Game/StopAndBreathe/Blueprints/SaveGameOMIG.anxietyDensityValue` (`self.anxietyDensityValue`) (`self.As Save Game OMIG`))))
    (:`then_4`
      (if (not (`KismetMathLibrary.EqualExactly_VectorVector` (`self.atriumSpawnLocation`) (`/Game/StopAndBreathe/Blueprints/SaveGameOMIG.atriumSpawnLocation` (`self.As Save Game OMIG`))))
        (set `/Game/StopAndBreathe/Blueprints/SaveGameOMIG.atriumSpawnLocation` (`self.atriumSpawnLocation`) (`self.As Save Game OMIG`))))
    (:`then_5`
      (if (not (== (`self.atriumFirstTimeCompleted?`) (`/Game/StopAndBreathe/Blueprints/SaveGameOMIG.atriumFirstTimeCompleted?` (`self.As Save Game OMIG`))))
        (set `/Game/StopAndBreathe/Blueprints/SaveGameOMIG.atriumFirstTimeCompleted?` (`self.atriumFirstTimeCompleted?`) (`self.As Save Game OMIG`))))
    (:`then_6`
      (`GameplayStatics.SaveGameToSlot` (`self.As Save Game OMIG`) "SaveGameOMIG"))))

(fn `SetData`
  (params (SaveGame :type "/Game/StopAndBreathe/Blueprints/SaveGameOMIG Object Reference") (sceneChange :type Boolean) (atriumAnxietyValue :type "Float (double-precision)") (currentLevel :type String) (starsCollected :type Integer) (atriumSpawnLocation :type "Vector Structure") (anxietyDensityValue :type "Float (double-precision)"))
  (set `self.As Save Game OMIG` SaveGame)
  (set `self.sceneChange` sceneChange)
  (set `self.atriumAnxietyValue` atriumAnxietyValue)
  (set `self.currentLevel` currentLevel)
  (set `self.starsCollected` starsCollected)
  (set `self.atriumSpawnLocation` atriumSpawnLocation)
  (set `self.anxietyDensityValue` anxietyDensityValue))