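; BP_Button is a pressure-plate style button that sends interaction messages to its AttachedObjects when actors overlap its box.
; It activates them on each overlap while active and cancels them once no tracked actors remain.
; ActivateObject restores the original material over the blocker one set at construction and stops audio.
; Tick and overlap events toggle an outline to show where a held BP_PickeableBox can snap.
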(event `self.ReceiveBeginPlay`
  (set `self.StartingScale` (`SceneComponent.K2_GetComponentScale` (`self.StaticMesh`))))

(event `self.Box.OnComponentBeginOverlap`
  (params (OverlappedComponent :type "PrimitiveComponent Object Reference") (OtherActor :type "Actor Object Reference") (OtherComp :type "PrimitiveComponent Object Reference") (OtherBodyIndex :type Integer) (bFromSweep :type Boolean) (SweepResult :type "HitResult Structure (by ref)"))
  (if (and (`GameplayStatics.ObjectIsA` OtherActor "/Script/Engine.Actor") (!= self OtherActor) (`self.isActive`))
    (`KismetArrayLibrary.Array_Add` (`self.OverlappingActors`) OtherActor)
    (for _array_element (`self.AttachedObjects`)
      (message `/Game/StopAndBreathe/Blueprints/Interfaces/BPI_Interactable.ActivateInteraction` _array_element)
      (if (`GameplayStatics.ObjectIsA` OtherActor)
        (`SceneComponent.SetVisibility` (`self.BoxOutline`) false false)))))

(event `self.Box.OnComponentEndOverlap`
  (params (OverlappedComponent :type "PrimitiveComponent Object Reference") (OtherActor :type "Actor Object Reference") (OtherComp :type "PrimitiveComponent Object Reference") (OtherBodyIndex :type Integer))
  (bind _overlappingactors (`self.OverlappingActors`))
  (if (`GameplayStatics.ObjectIsA` OtherActor "/Script/Engine.Actor")
    (`KismetArrayLibrary.Array_RemoveItem` _overlappingactors OtherActor)
    (if (`KismetArrayLibrary.Array_IsEmpty` _overlappingactors)
      (`KismetArrayLibrary.Array_Clear` (`self.OverlappingActors`))
      (for _array_element (`self.AttachedObjects`)
        (message `/Game/StopAndBreathe/Blueprints/Interfaces/BPI_Interactable.CancelInteraction` _array_element)
        (if (`GameplayStatics.ObjectIsA` OtherActor "/Game/StopAndBreathe/Blueprints/Interactables/BP_PickeableBox.BP_PickeableBox_C")
          (`SceneComponent.SetVisibility` (`self.BoxOutline`) true false))))))

(event `/Game/StopAndBreathe/Blueprints/Interfaces/BPI_Interactable.ActivateObject`
  (set `self.isActive` true)
  (`PrimitiveComponent.SetMaterial` (`self.StaticMesh`) 0 (`self.TrueMat`))
  (`AudioComponent.Stop` (`self.Audio`)))

(event `/Game/StopAndBreathe/Blueprints/Interfaces/BPI_Interactable.DeactivateObject`
  (set `self.isActive` false))

(event `self.ReceiveTick`
  (params (DeltaSeconds :type "Float (single-precision)"))
  (bind _overlappingactors (`PrimitiveComponent.GetOverlappingActors` (`self.SnapRadius`) "/Game/StopAndBreathe/Blueprints/Interactables/BP_PickeableBox.BP_PickeableBox_C"))
  ;[1 1 1] Check if box is in snap radius, then turn on or off the outline
  (if (`KismetArrayLibrary.Array_IsNotEmpty` _overlappingactors)
    (bind _asbp_pickeable_box (cast `/Game/StopAndBreathe/Blueprints/Interactables/BP_PickeableBox` (`|GetArrayItem` _overlappingactors)))
    (if (`/Game/StopAndBreathe/Blueprints/Interactables/BP_PickeableBox.IsBeingHeld` _asbp_pickeable_box)
      (`SceneComponent.SetVisibility` (`self.BoxOutline`) true false))
    (else
      (`SceneComponent.SetVisibility` (`self.BoxOutline`) false false))))

(fn `UserConstructionScript`
  (set `self.TrueMat` (`PrimitiveComponent.GetMaterial` (`self.StaticMesh`) 0))
  (`PrimitiveComponent.SetMaterial` (`self.StaticMesh`) 0 "/Game/StopAndBreathe/Materials/Shaders/BAOBlocker.BAOBlocker"))