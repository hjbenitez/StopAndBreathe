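; Tree actor for StopAndBreathe that starts in a placeholder look and gains its real materials when activated.
; The construction script applies the bark and leaves materials, caches them in TrueMats, then overrides the first slot with BAOBlocker and clears the second.
; ActivateObject restores each cached material to its slot on the Tree mesh.
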(event `/Game/StopAndBreathe/Blueprints/Interfaces/BPI_Interactable.ActivateObject`
  (for (_array_element _array_index) (`self.TrueMats`)
    (`PrimitiveComponent.SetMaterial` (`self.Tree`) _array_index _array_element)))

(fn `UserConstructionScript`
  (`|ExecutionSequence`
    (:`then_1`
      (`PrimitiveComponent.SetMaterial` (`self.Tree`) 0 "/Game/StopAndBreathe/Assets/Trees/NormalTree_Bark.NormalTree_Bark")
      (`PrimitiveComponent.SetMaterial` (`self.Tree`) 1 "/Game/StopAndBreathe/Assets/Trees/NormalTree_Leaves.NormalTree_Leaves")
      (set `self.TrueMats` (`MeshComponent.GetMaterials` (`self.Tree`))))
    (:`then_2`
      (`PrimitiveComponent.SetMaterial` (`self.Tree`) 0 "/Game/StopAndBreathe/Materials/Shaders/BAOBlocker.BAOBlocker")
      (`PrimitiveComponent.SetMaterial` (`self.Tree`) 1 "/Game/StopAndBreathe/Materials/Shaders/Null.Null"))))