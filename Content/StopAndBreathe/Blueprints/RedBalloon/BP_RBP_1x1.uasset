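; BP_RBP_1x1 is a red balloon platform Blueprint that responds to an inhale, exhale or off state set through ObjectFunction.
; BeginPlay stores the platform's world location, then initializes and inflates the balloon.
; Each Tick switches on that state to go down, go up or turn off, re-inflating in both moving states, then lifts the balloon.
; Debug prints show the fan state and hit component, and BalloonPull is unwired.
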(event `self.ReceiveBeginPlay`
  (set `self.position` (`SceneComponent.K2_GetComponentLocation` (`self.Platform`)))
  (`self.Initialization`)
  (`self.inflateBalloon`))

(event `self.ReceiveTick`
  (params (DeltaSeconds :type "Float (single-precision)"))
  (`KismetSystemLibrary.PrintString` (`|GetEnumeratorNameAsString` (`self.fanState`)))
  (`|ExecutionSequence`
    (:`then_0`
      (switch `/Game/StopAndBreathe/Blueprints/Interactables/ENUM_InteractableStates` (`self.intertactable`)
        (:`NewEnumerator2`
          (`self.Off`))
        (:`NewEnumerator0`
          (`self.GoDown`)
          (`self.inflateBalloon` :!label _label))
        (:`NewEnumerator1`
          (`self.GoUp`)
          (goto _label))))
    (:`then_1`
      (`self.LiftBalloon`))))

(event `/Game/StopAndBreathe/Blueprints/Interfaces/BPI_Interactable.ObjectFunction`
  (params (NewParam :type "/Game/StopAndBreathe/Blueprints/Interactables/ENUM_InteractableStates Enum" :default "NewEnumerator2"))
  (set `self.intertactable` NewParam))

(event `self.ReceiveHit`
  (params (MyComp :type "PrimitiveComponent Object Reference") (Other :type "Actor Object Reference") (OtherComp :type "PrimitiveComponent Object Reference") (bSelfMoved :type Boolean) (HitLocation :type "Vector Structure") (HitNormal :type "Vector Structure") (NormalImpulse :type "Vector Structure") (Hit :type "HitResult Structure (by ref)"))
  (`KismetSystemLibrary.PrintString` (`KismetSystemLibrary.GetDisplayName` MyComp)))

(fn `UserConstructionScript`
  (`parent.UserConstructionScript`))