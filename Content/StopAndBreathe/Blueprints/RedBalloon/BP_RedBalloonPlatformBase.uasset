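; Base for a red balloon platform that rises and descends between two marker heights and gets pushed or drawn horizontally by fans.
; Initialization caches the height limits, creates the balloon's dynamic material and attaches an optional breathing terminal to the platform.
; Platform height drives the material's inflation, while fan inhale or exhale offsets balloon and platform along a rounded direction.
; BalloonPull sets per-axis pull flags with hysteresis, but its movement nodes are disconnected.
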(fn `Add Actors`
  (if (`KismetSystemLibrary.IsValid` (`self.breathingTerminalOnPlatform`))
    (`self.K2_AttachToComponent` (`self.breathingTerminalOnPlatform`) (`self.Platform`) "None" "KeepWorld" "KeepWorld" "KeepWorld" true)))

(fn `BalloonPull`
  (locals (balloonPosition :type "Vector2D Structure"))
  (bind _balloonposition_x (`KismetMathLibrary.BreakVector2D` (`local.balloonPosition`)))
  (bind _balloonposition_x_2 (`KismetMathLibrary.BreakVector2D` (`local.balloonPosition`)))
  (bind _balloonposition_x_3 (`KismetMathLibrary.BreakVector2D` (`local.balloonPosition`)))
  (bind _balloonposition_x_4 (`KismetMathLibrary.BreakVector2D` (`local.balloonPosition`)))
  (bind (_balloonposition_x_5 _balloonposition_y) (`KismetMathLibrary.BreakVector2D` (`local.balloonPosition`)))
  (bind (_balloonposition_x_6 _balloonposition_y_2) (`KismetMathLibrary.BreakVector2D` (`local.balloonPosition`)))
  (bind (_balloonposition_x_7 _balloonposition_y_3) (`KismetMathLibrary.BreakVector2D` (`local.balloonPosition`)))
  (bind (_balloonposition_x_8 _balloonposition_y_4) (`KismetMathLibrary.BreakVector2D` (`local.balloonPosition`)))
  (set `local.balloonPosition` (`KismetMathLibrary.Conv_VectorToVector2D` (- (`SceneComponent.K2_GetComponentLocation` (`self.Platform`)) (`SceneComponent.RelativeLocation` (`self.balloon`)))))
  (`|ExecutionSequence`
    (:`then_0`
      (`|ExecutionSequence`
        (:`then_0`
          (if (or (`self.balloonForwardPullX`) (`self.balloonBackwardPullX`))
            _))
        (:`then_1`
          (if (or (`self.balloonForwardPullY`) (`self.balloonBackwardPullY`))
            _))))
    (:`then_1`
      (`|ExecutionSequence`
        (:`then_0`
          (if (> _balloonposition_x_2 (`self.balloonPullThreshold`))
            (set `self.balloonForwardPullX` true)
            (set `self.balloonBackwardPullX` false)))
        (:`then_1`
          (if (< _balloonposition_x (* -1.0 (`self.balloonPullThreshold`)))
            (set `self.balloonForwardPullX` false)
            (set `self.balloonBackwardPullX` true)))
        (:`then_2`
          (if (and (< _balloonposition_x_3 (`self.balloonStopPullThreshold`)) (> _balloonposition_x_4 (* -1.0 (`self.balloonStopPullThreshold`))))
            (set `self.balloonForwardPullX` false)
            (set `self.balloonBackwardPullX` false)))))
    (:`then_2`
      (`|ExecutionSequence`
        (:`then_0`
          (if (> _balloonposition_y_4 (`self.balloonPullThreshold`))
            (set `self.balloonForwardPullY` true)
            (set `self.balloonBackwardPullY` false)))
        (:`then_1`
          (if (< _balloonposition_y_2 (* -1.0 (`self.balloonPullThreshold`)))
            (set `self.balloonForwardPullY` false)
            (set `self.balloonBackwardPullY` true)))
        (:`then_2`
          (if (and (< _balloonposition_y_3 (`self.balloonStopPullThreshold`)) (> _balloonposition_y (* -1.0 (`self.balloonStopPullThreshold`))))
            (set `self.balloonForwardPullY` false)
            (set `self.balloonBackwardPullY` false)))))))

(fn `ClampVelocity`
  (params (Platform :type "PrimitiveComponent Object Reference"))
  (`PrimitiveComponent.SetPhysicsLinearVelocity` Platform (`KismetMathLibrary.ClampVectorSize` (`SceneComponent.GetComponentVelocity` Platform) 0.0 (`self.moveSpeed`)) false "None"))

(fn `GoDown`
  (bind (_returnvalue_x _returnvalue_y _returnvalue_z) (`KismetMathLibrary.BreakVector` (`SceneComponent.K2_GetComponentLocation` (`self.Platform`))))
  (if (> _returnvalue_z (`self.minHeight`))
    (`SceneComponent.K2_AddWorldOffset` (`self.Platform`) (`KismetMathLibrary.MakeVector` 0.0 0.0 (* (`self.moveSpeed`) -1.0)) false false)))

(fn `GoUp`
  (bind (_returnvalue_x _returnvalue_y _returnvalue_z) (`KismetMathLibrary.BreakVector` (`SceneComponent.K2_GetComponentLocation` (`self.Platform`))))
  (if (< _returnvalue_z (`self.maxHeight`))
    (`SceneComponent.K2_AddWorldOffset` (`self.Platform`) (`KismetMathLibrary.MakeVector` 0.0 0.0 (`self.moveSpeed`)) false false)))

(fn `inflateBalloon`
  (bind (_returnvalue_x _returnvalue_y _returnvalue_z) (`KismetMathLibrary.BreakVector` (`SceneComponent.K2_GetComponentLocation` (`self.Platform`))))
  (set `self.balloonHeight` _returnvalue_z)
  (`MaterialInstanceDynamic.SetScalarParameterValue` (`self.balloonMaterial`) "inflateAmount" (+ -5.5 (* (- 25.0 -5.5) (/ (- (`self.balloonHeight`) (`self.minHeight`)) (- (`self.maxHeight`) (`self.minHeight`)))))))

(fn `Initialization`
  (bind (_returnvalue_x _returnvalue_y _returnvalue_z) (`KismetMathLibrary.BreakVector` (`SceneComponent.K2_GetComponentLocation` (`self.maxPoint`))))
  (bind (_returnvalue_x_2 _returnvalue_y_2 _returnvalue_z_2) (`KismetMathLibrary.BreakVector` (`SceneComponent.K2_GetComponentLocation` (`self.minPoint`))))
  (set `self.minHeight` _returnvalue_z_2)
  (set `self.maxHeight` _returnvalue_z)
  (bind _returnvalue (`PrimitiveComponent.CreateDynamicMaterialInstance` (`self.balloon`) 0 "/Game/StopAndBreathe/Materials/Shaders/Balloon.Balloon" "None"))
  (set `self.balloonMaterial` _returnvalue)
  (`self.Add Actors`))

(fn `LiftBalloon`
  (`PrimitiveComponent.AddForce` (`self.balloon`) (0.0 0.0 800.0) "None" true))

(fn `Off`)

(fn `Push Fan`
  (params (fanLocation :type "Vector Structure") (fanState :type "/Game/StopAndBreathe/Blueprints/Interactables/ENUM_InteractableStates Enum" :default "NewEnumerator2"))
  (bind (_fandirection_x _fandirection_y) (`KismetMathLibrary.BreakVector2D` (`self.fanDirection`)))
  (bind _fanblowingvalue (`self.fanBlowingValue`))
  (bind _returnvalue (* (`self.pushSpeed`) 1.5))
  (bind _returnvalue_2 (* _fandirection_x _returnvalue _fanblowingvalue))
  (bind _returnvalue_3 (* _fandirection_y _returnvalue _fanblowingvalue))
  (bind (_returnvalue_x _returnvalue_y) (`KismetMathLibrary.BreakVector` (`KismetMathLibrary.Normal` (- (`SceneComponent.K2_GetComponentLocation` (`self.Platform`)) fanLocation))))
  (if (`|EnumInequality` fanState (`self.fanState`))
    (`|ExecutionSequence`
      (:`then_0`
        (set `self.balloonForwardPullX` false)
        (set `self.balloonBackwardPullX` false))
      (:`then_1`
        (set `self.balloonForwardPullY` false)
        (set `self.balloonBackwardPullY` false))
      (:`then_2`
        (bind _output_get (set `self.fanState` fanState :!label _label))
        (set `self.fanDirection` (`KismetMathLibrary.MakeVector2D` (`KismetMathLibrary.Conv_IntToDouble` (`KismetMathLibrary.Round` _returnvalue_x)) (`KismetMathLibrary.Conv_IntToDouble` (`KismetMathLibrary.Round` _returnvalue_y))))
        (switch `/Game/StopAndBreathe/Blueprints/Interactables/ENUM_InteractableStates` _output_get
          (:`NewEnumerator0`
            (set `self.fanBlowingValue` -1))
          (:`NewEnumerator1`
            (set `self.fanBlowingValue` 1)))
        (`SceneComponent.K2_AddWorldOffset` (`self.balloon`) (`KismetMathLibrary.MakeVector` _returnvalue_2 _returnvalue_3) true false)
        (`SceneComponent.K2_AddWorldOffset` (`self.Platform`) (`KismetMathLibrary.MakeVector` _returnvalue_2 _returnvalue_3) true false)))
    (else
      (goto _label))))

(fn `UserConstructionScript`)