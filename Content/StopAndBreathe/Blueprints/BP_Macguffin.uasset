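; BP_Macguffin is a collectible actor that the third-person character picks up by overlapping it, adding one to the stars-collected count.
; BeginPlay caches the GI_StoreInformation game instance, which holds the running StarsCollected total.
; On pickup it loads or creates the SaveGameOMIG save, copies the incremented total into it, saves the slot, prints the count and destroys itself.
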(event `self.ReceiveBeginPlay`
  (bind _asgi_store_information (cast `/Game/StopAndBreathe/Blueprints/GI_StoreInformation` (`GameplayStatics.GetGameInstance`)))
  (set `self.As GI Store Information` _asgi_store_information))

(event `self.ReceiveActorBeginOverlap`
  (params (OtherActor :type "Actor Object Reference"))
  (bind _as_gi_store_information (`self.As GI Store Information`))
  (if (`GameplayStatics.ObjectIsA` OtherActor "/Game/ThirdPerson/Blueprints/BP_ThirdPersonCharacter.BP_ThirdPersonCharacter_C")
    (bind _returnvalue (`GameplayStatics.DoesSaveGameExist` "SaveGameOMIG"))
    (if _returnvalue
      (bind _returnvalue_2 (`GameplayStatics.LoadGameFromSlot` "SaveGameOMIG"))
      (bind _assave_game_omig (cast `/Game/StopAndBreathe/Blueprints/SaveGameOMIG` _returnvalue_2)
        (:`then`
          (bind _output_get (set `self.As Save Game OMIG` _assave_game_omig))
          (bind _output_get_2 (set `/Game/StopAndBreathe/Blueprints/GI_StoreInformation.starsCollected` (+ (`/Game/StopAndBreathe/Blueprints/GI_StoreInformation.starsCollected` _as_gi_store_information) 1) _as_gi_store_information :!label _label))
          (bind _output_get_3 (set `/Game/StopAndBreathe/Blueprints/SaveGameOMIG.StarsCollected` _output_get_2 _output_get))
          (`GameplayStatics.SaveGameToSlot` (`self.As Save Game OMIG`) "SaveGameOMIG")
          (`KismetSystemLibrary.PrintString` (`KismetStringLibrary.Concat_StrStr` "yoyoyoyoyoy" (`KismetStringLibrary.Conv_IntToString` _output_get_3)))
          (`self.K2_DestroyActor`))
        (:`CastFailed`
          (`KismetSystemLibrary.PrintString` "fuck")))
      (else
        (bind _returnvalue_3 (`GameplayStatics.CreateSaveGameObject` "/Game/StopAndBreathe/Blueprints/SaveGameOMIG.SaveGameOMIG_C"))
        (set `self.As Save Game OMIG` _returnvalue_3)
        (goto _label)))))

(fn `UserConstructionScript`)