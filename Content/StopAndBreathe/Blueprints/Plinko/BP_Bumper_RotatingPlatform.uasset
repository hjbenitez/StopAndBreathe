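; Plinko bumper platform that rotates with the breathing state and knocks pickable boxes away on overlap.
; ObjectFunction maps Inhale, Exhale and Off to rotation direction; Tick turns the mesh on a selectable axis and feeds faster gear rotation to its AnimBP.
; Overlapping boxes get a randomized cone impulse with a pinball sound.
; ActivateObject stops anxiety audio and swaps the blocker material to blue; older rotation logic is unused.
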(event `self.ReceiveBeginPlay`
  (`|ExecutionSequence`
    (:`then_0`
      (`PrimitiveComponent.SetMaterial` (`self.Platform`) 0 "/Game/StopAndBreathe/Materials/Shaders/BAOBlocker.BAOBlocker")
      (bind _asabp_bumper_rotating_plat (cast `/Game/StopAndBreathe/Assets/mechanic_assets/RotatingPlatform/ABP_BumperRotatingPlat` (`SkeletalMeshComponent.GetAnimInstance` (`self.Platform`))))
      (set `self.Reg ABP Ref` _asabp_bumper_rotating_plat))
    (:`then_1`
      (set `self.GearRotationSpeed` (* (`self.RotationSpeed`) 3.0)))))

(event `Rotate Platform Old`
  (params (Direction :type Integer :default 1))
  ;[1 1 1 1 100] Deprecated
  ;;[1 0.1982 0.8249] Rotate the Platform, if the Platform is Not Already Rotating
  (if true
    _))

(event `self.ReceiveTick`
  (params (DeltaSeconds :type "Float (single-precision)"))
  (set `self.Delta Seconds` DeltaSeconds)
  (if (`|EnumInequality` (`self.CurrentState`) "NewEnumerator2")
    (bind _output_get (set `self.CurrentRotation` (+ (`self.CurrentRotation`) (* (`self.RotationRate`) (`self.Delta Seconds`)))))
    (`SceneComponent.K2_SetRelativeRotation` (`self.Platform`) (select `/Game/StopAndBreathe/Blueprints/E_RotationAxis` (`self.RotateAlong`) :`NewEnumerator1` (`KismetMathLibrary.MakeRotator` 0.0 _output_get) :`NewEnumerator2` (`KismetMathLibrary.MakeRotator` 0.0 0.0 _output_get) :`NewEnumerator0` (`KismetMathLibrary.MakeRotator` _output_get)) false false)
    (`self.PlayGearAnim`)))

(event `self.ObjectFunction`
  (params (NewParam :type "/Game/StopAndBreathe/Blueprints/Interactables/ENUM_InteractableStates Enum" :default "NewEnumerator2"))
  (bind _output_get (set `self.CurrentState` NewParam))
  (switch `/Game/StopAndBreathe/Blueprints/Interactables/ENUM_InteractableStates` _output_get
    (:`NewEnumerator2`
      (set `self.RotationRate` 0.0))
    (:`NewEnumerator0`
      (set `self.RotationRate` (* (`self.RotationSpeed`) -1.0)))
    (:`NewEnumerator1`
      (set `self.RotationRate` (`self.RotationSpeed`)))))

(event `self.ActivateObject`
  (`AudioComponent.Stop` (`self.AnxietyAudio`))
  (`PrimitiveComponent.SetMaterial` (`self.Platform`) 0 "/Game/StopAndBreathe/Materials/Development/Blue_Mat.Blue_Mat"))

(event `self.ReceiveActorBeginOverlap`
  (params (OtherActor :type "Actor Object Reference"))
  (bind _asbp_pickeable_box (cast `/Game/StopAndBreathe/Blueprints/Interactables/BP_PickeableBox` OtherActor))
  (`KismetSystemLibrary.PrintString` "Hello")
  (`PrimitiveComponent.AddImpulse` (`/Game/StopAndBreathe/Blueprints/Interactables/BP_BaseInteractable.StaticMesh` _asbp_pickeable_box) (* (`KismetMathLibrary.RandomUnitVectorInConeInDegrees` (`KismetMathLibrary.GetDirectionUnitVector` (`SceneComponent.K2_GetComponentLocation` (`self.Platform`)) (`self.K2_GetActorLocation` OtherActor)) 30.0) (`self.BumperForce`)) "None" false)
  (`GameplayStatics.SpawnSound2D` "/Game/Audio/MetaSounds/MS_PinballRing.MS_PinballRing" 0.2 1.0 0.0 null))

(fn `PlayGearAnim`
  (switch `/Game/StopAndBreathe/Blueprints/Interactables/ENUM_InteractableStates` (`self.CurrentState`)
    (:`NewEnumerator2`
      (bind _output_get (set `self.GearRotation` (+ (`self.GearRotation`) 0.0)))
      (`/Game/StopAndBreathe/Assets/mechanic_assets/RotatingPlatform/ABP_BumperRotatingPlat.RotationEvent` (`self.Reg ABP Ref`) _output_get))
    (:`NewEnumerator0`
      (bind _output_get_2 (set `self.GearRotation` (+ (`self.GearRotation`) (* (`self.GearRotationSpeed`) (`self.Delta Seconds`)))))
      (`/Game/StopAndBreathe/Assets/mechanic_assets/RotatingPlatform/ABP_BumperRotatingPlat.RotationEvent` (`self.Reg ABP Ref`) _output_get_2))
    (:`NewEnumerator1`
      (bind _output_get_3 (set `self.GearRotation` (- (`self.GearRotation`) (* (`self.GearRotationSpeed`) (`self.Delta Seconds`)))))
      (`/Game/StopAndBreathe/Assets/mechanic_assets/RotatingPlatform/ABP_BumperRotatingPlat.RotationEvent` (`self.Reg ABP Ref`) _output_get_3))))

(fn `UserConstructionScript`)