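; Plinko bumper actor that knocks pickeable boxes away when they overlap it, like a pinball bumper.
; On overlap with a BP_PickeableBox, it applies an impulse to the box's mesh, scaled by BumperForce.
; The impulse points from the cylinder toward the box, randomized within a cone to vary the bounce.
; Each hit also plays a 2D pinball ring sound and prints a debug string.
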(event `self.ReceiveActorBeginOverlap`
  (params (OtherActor :type "Actor Object Reference"))
  (bind _asbp_pickeable_box (cast `/Game/StopAndBreathe/Blueprints/Interactables/BP_PickeableBox` OtherActor))
  (`KismetSystemLibrary.PrintString` "Hello")
  (`PrimitiveComponent.AddImpulse` (`/Game/StopAndBreathe/Blueprints/Interactables/BP_BaseInteractable.StaticMesh` _asbp_pickeable_box) (* (`KismetMathLibrary.RandomUnitVectorInConeInDegrees` (`KismetMathLibrary.GetDirectionUnitVector` (`SceneComponent.K2_GetComponentLocation` (`self.Cylinder`)) (`self.K2_GetActorLocation` OtherActor)) 30.0) (`self.BumperForce`)) "None" false)
  (`GameplayStatics.SpawnSound2D` "/Game/Audio/MetaSounds/MS_PinballRing.MS_PinballRing" 0.2 1.0 0.0 null))

(fn `UserConstructionScript`)