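; BP_BAOActivator is a volume that switches the BAO objects inside its collision component from inactive to active.
; On BeginPlay it sends a deactivate message to overlapping actors implementing BPI_Interactable.
; ActivateBAOs sends those actors the activate message, then makes overlapping components tagged "Bphase" visible with BlockAll collision.
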(event `ActivateBAOs`
  (`|ExecutionSequence`
    (:`then_0`
      (for _array_element (`PrimitiveComponent.GetOverlappingActors` (`self.CollisionComponent`) "/Script/Engine.Actor")
        (if (`KismetSystemLibrary.DoesImplementInterface` _array_element "/Game/StopAndBreathe/Blueprints/Interfaces/BPI_Interactable.BPI_Interactable_C")
          (message `/Game/StopAndBreathe/Blueprints/Interfaces/BPI_Interactable.ActivateObject` _array_element))))
    (:`then_1`
      (for _array_element_2 (`PrimitiveComponent.GetOverlappingComponents` (`self.CollisionComponent`))
        (if (`ActorComponent.ComponentHasTag` _array_element_2 "Bphase")
          (`KismetSystemLibrary.PrintString` (`KismetSystemLibrary.GetDisplayName` _array_element_2))
          (`PrimitiveComponent.SetCollisionProfileName` _array_element_2 "BlockAll" false)
          (`SceneComponent.SetVisibility` _array_element_2 true false))))))

(event `self.ReceiveBeginPlay`
  (for _array_element (`PrimitiveComponent.GetOverlappingActors` (`self.CollisionComponent`) "/Script/Engine.Actor")
    (if (`KismetSystemLibrary.DoesImplementInterface` _array_element "/Game/StopAndBreathe/Blueprints/Interfaces/BPI_Interactable.BPI_Interactable_C")
      (message `/Game/StopAndBreathe/Blueprints/Interfaces/BPI_Interactable.DeactivateObject` _array_element))))

(fn `UserConstructionScript`)