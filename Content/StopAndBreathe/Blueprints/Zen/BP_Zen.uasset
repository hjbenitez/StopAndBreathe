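; BP_Zen is a flying companion that follows the player or settles on a shoulder, depending on ZenMode.
; It registers as a follower on BeginPlay, then runs two looping timers instead of Tick: random offset and movement updates.
; Movement queries the player through messages, picks the nearer left or right point, and interpolates rotation and FloatingPawnMovement velocity using player-based speed.
; Following adds the random offset, while sitting zeroes velocity near the shoulder.
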(event `self.ReceiveBeginPlay`
  (bind _output_get (set `self.player` (`GameplayStatics.GetPlayerCharacter` 0)))
  (`/Engine/EditorBlueprintResources/StandardMacros.IsValid` _output_get
    (:`Is Valid`
      (message `/Game/StopAndBreathe/Blueprints/Zen/BPI_ZenTalk.AddFollower` _output_get self)
      (bind _returnvalue (`KismetSystemLibrary.K2_SetTimerDelegate` (delegate `GenerateRandomOffsetTick`) (`self.randomOffsetTickRate`) true))
      (set `self.randomOffsetTimer` _returnvalue)
      (bind _returnvalue_2 (`KismetSystemLibrary.K2_SetTimerDelegate` (delegate `VelocityUpdateTick`) (`self.velocityUpdateTickRate`) true))
      (set `self.velocityUpdateTimer` _returnvalue_2))))

(event `GenerateRandomOffsetTick`
  (set `self.randomOffset` (`self.GenerateRandomOffset`)))

(event `VelocityUpdateTick`
  (bind _floatingpawnmovement (`self.FloatingPawnMovement`))
  (bind _floatingpawnmovement_2 (`self.FloatingPawnMovement`))
  (switch `/Game/StopAndBreathe/Blueprints/Zen/E_ZenMode` (`self.zenMode`)
    (:`NewEnumerator0`
      (bind (_rot _leftbehind _rightbehind _speed) (message `/Game/StopAndBreathe/Blueprints/Zen/BPI_ZenTalk.FlyingPlayerQuery` (`self.player`)))
      (`|ExecutionSequence`
        (:`then_0`
          (`self.K2_SetActorRotation` (`KismetMathLibrary.RInterpTo` (`self.K2_GetActorRotation`) _rot (`self.velocityUpdateTickRate`) (`self.rinterpSpeed`))))
        (:`then_1`
          (bind _returnvalue (+ (* _speed 0.9) 150.0))
          (set `MovementComponent.Velocity` (`KismetMathLibrary.VInterpTo` (`MovementComponent.Velocity` _floatingpawnmovement) (* (`KismetMathLibrary.Normal` (- (+ (select `bool` (`self.GetLeftRight` _leftbehind _rightbehind) :`false` _leftbehind :`true` _rightbehind) (`self.randomOffset`)) (`self.K2_GetActorLocation`))) (`KismetMathLibrary.SelectFloat` 100.0 _returnvalue (< _returnvalue 200.0))) (`self.velocityUpdateTickRate`) (`self.vinterpSpeed`)) _floatingpawnmovement))))
    (:`NewEnumerator1`
      (bind (_rot_2 _leftshoulder _rightshoulder _speed_2) (message `/Game/StopAndBreathe/Blueprints/Zen/BPI_ZenTalk.SittingQuery` (`self.player`)))
      (`|ExecutionSequence`
        (:`then_0`
          (`self.K2_SetActorRotation` (`KismetMathLibrary.RInterpTo` (`self.K2_GetActorRotation`) _rot_2 (`self.velocityUpdateTickRate`) (`self.rinterpSpeed`))))
        (:`then_1`
          (bind _returnvalue_2 (select `bool` (`self.GetLeftRight` _leftshoulder _rightshoulder) :`false` _leftshoulder :`true` _rightshoulder))
          (bind _returnvalue_3 (+ (* _speed_2 0.9) 150.0))
          (set `MovementComponent.Velocity` (`KismetMathLibrary.VInterpTo` (`MovementComponent.Velocity` _floatingpawnmovement_2) (* (`KismetMathLibrary.Normal` (- _returnvalue_2 (`self.K2_GetActorLocation`))) (`KismetMathLibrary.SelectFloat` 100.0 _returnvalue_3 (< _returnvalue_3 200.0))) (`self.velocityUpdateTickRate`) (`self.vinterpSpeed`)) _floatingpawnmovement_2)
          (if (< (`KismetMathLibrary.VSize` (- _returnvalue_2 (`self.K2_GetActorLocation`))) 5.0)
            (set `MovementComponent.Velocity` (0.0 0.0 0.0) (`self.FloatingPawnMovement`))))))))

(fn `FlyingPlayerQuery`
  (returns (rot :type "Rotator Structure") (leftBehind :type "Vector Structure") (rightBehind :type "Vector Structure") (speed :type "Float (double-precision)"))
  (return (struct) (0.0 0.0 0.0) (0.0 0.0 0.0) 0.0))

(fn `GenerateRandomOffset`
  (returns (newOffset :type "Vector Structure"))
  (bind (_randomoffsetminmax_x _randomoffsetminmax_y _randomoffsetminmax_z) (`KismetMathLibrary.BreakVector` (`self.randomOffsetMinMax`)))
  (return (`KismetMathLibrary.MakeVector` (`KismetMathLibrary.RandomFloatInRange` (* _randomoffsetminmax_x -1) _randomoffsetminmax_x) (`KismetMathLibrary.RandomFloatInRange` (* _randomoffsetminmax_y -1) _randomoffsetminmax_y) (`KismetMathLibrary.RandomFloatInRange` (* _randomoffsetminmax_z -1) _randomoffsetminmax_z))))

(fn `GetLeftRight`
  (params (left :type "Vector Structure") (right :type "Vector Structure"))
  (returns (`goRight?` :type Boolean))
  (bind _returnvalue (`self.K2_GetActorLocation`))
  (return (> (`KismetMathLibrary.VSize` (- _returnvalue left)) (`KismetMathLibrary.VSize` (- _returnvalue right)))))

(fn `SittingQuery`
  (returns (rot :type "Rotator Structure") (leftShoulder :type "Vector Structure") (rightShoulder :type "Vector Structure") (speed :type "Float (double-precision)"))
  (return (struct) (0.0 0.0 0.0) (0.0 0.0 0.0) 0.0))

(fn `UserConstructionScript`)