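; BP_BreathingTrigger177 is a spotlit breathing spot that sets InBreathingTrigger on BP_ThirdPersonCharacter177 while the player overlaps it.
; It stores the overlapping actor and, until its Done flag is true, toggles that player flag on enter and exit.
; Once Done is set, Tick clears the flag, lerps the spotlight from its current intensity toward zero over two seconds, then destroys the actor.
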(event `Remove Trigger`
  ;[1 0.07961 0.02985] Remove This Actor
  (`self.K2_DestroyActor`))

(event `self.ReceiveActorBeginOverlap`
  (params (OtherActor :type "Actor Object Reference"))
  ;[1 0.2984 0.8739] Tell The Player BP That They Have Entered/Left A Breathing Spot
  (bind _output_get (set `self.Other Actor` OtherActor))
  (bind _asbp_third_person_character_177 (cast `/Game/ThirdPerson/Blueprints/BP_ThirdPersonCharacter177` _output_get))
  (if (not (`self.done`))
    (set `/Game/ThirdPerson/Blueprints/BP_ThirdPersonCharacter177.inBreathingTrigger` true _asbp_third_person_character_177)))

(event `self.ReceiveActorEndOverlap`
  (params (OtherActor :type "Actor Object Reference"))
  ;[1 0.2984 0.8739] Tell The Player BP That They Have Entered/Left A Breathing Spot
  (bind _output_get (set `self.Other Actor` OtherActor))
  (bind _asbp_third_person_character_177 (cast `/Game/ThirdPerson/Blueprints/BP_ThirdPersonCharacter177` _output_get))
  (if (not (`self.done`))
    (set `/Game/ThirdPerson/Blueprints/BP_ThirdPersonCharacter177.inBreathingTrigger` false _asbp_third_person_character_177)))

(event `self.ReceiveTick`
  (params (DeltaSeconds :type "Float (single-precision)"))
  ;[1 0.981 0.2425] Remove The Spot With a Smooth Transistion (Decrease The Light Intensity)
  (if (`self.done`)
    (bind _asbp_third_person_character_177 (cast `/Game/ThirdPerson/Blueprints/BP_ThirdPersonCharacter177` (`self.Other Actor`)))
    (set `/Game/ThirdPerson/Blueprints/BP_ThirdPersonCharacter177.inBreathingTrigger` false _asbp_third_person_character_177)
    (bind _output_get (set `self.lightTimer` (+ (`self.lightTimer`) (`GameplayStatics.GetWorldDeltaSeconds`))))
    (`LightComponent.SetIntensity` (`self.SpotLight`) (`KismetMathLibrary.Lerp` (`LightComponentBase.Intensity` (`self.SpotLight`)) 0.0 (/ _output_get 2.0)))
    (if (>= (`self.lightTimer`) 2.0)
      (`self.Remove Trigger`))))

(fn `UserConstructionScript`)