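; Chase-scene monster that pursues the player along world Y, hidden until the player exits its trigger, which starts audio and chase music.
; A timed lerp first pulls it toward a point behind the player, ending early once within minimum distance.
; It then advances at constant rates, faster when far behind, slower when near; IsMonsterTooClose actually returns true when far.
; Touching the player stops it and snaps it to the Arrow.
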(event `self.ReceiveBeginPlay`
  (bind (_returnvalue_x _returnvalue_y) (`KismetMathLibrary.BreakVector` (`SceneComponent.K2_GetComponentLocation` (`self.Monster`))))
  (`SceneComponent.SetVisibility` (`self.Monster`) false false)
  (set `self.StartingMonsterYPos` _returnvalue_y)
  (set `self.MoveToTimer` (`self.InitialMoveToTimer`)))

(event `self.ReceiveTick`
  (params (DeltaSeconds :type "Float (single-precision)"))
  (set `self.Delta Seconds` DeltaSeconds)
  (if (and (`self.hasMonsterStarted?`) (> (`self.MoveToTimer`) 0.0))
    (bind _output_get (set `self.MoveToTimer` (- (`self.MoveToTimer`) (`self.Delta Seconds`))))
    (`KismetSystemLibrary.PrintString` (`KismetStringLibrary.Conv_DoubleToString` _output_get) true true (struct :`R` 1.0 :`B` 0.697584 :`A` 1.0))
    (`self.InitialMoveMonsterToPlayer`)
    (else
      ;[0.3281 0.3266 0.3035 0.885] Normal Monster Movement
      (if (`self.TouchedPlayer`)
        _
        (elif (and (`self.hasMonsterStarted?`) (<= (`self.MoveToTimer`) 0.0))
          (`self.Follow Player`))))))

(event `StartMonster`
  (set `self.hasMonsterStarted?` true)
  (`SceneComponent.SetVisibility` (`self.Monster`) true false))

(event `self.MonsterTrigger.OnComponentBeginOverlap`
  (params (OverlappedComponent :type "PrimitiveComponent Object Reference") (OtherActor :type "Actor Object Reference") (OtherComp :type "PrimitiveComponent Object Reference") (OtherBodyIndex :type Integer) (bFromSweep :type Boolean) (SweepResult :type "HitResult Structure (by ref)"))
  (if (`GameplayStatics.ObjectIsA` OtherActor "/Game/ThirdPerson/Blueprints/BP_ThirdPersonCharacter.BP_ThirdPersonCharacter_C")
    (bind _output_get (set `self.PlayerCharacter` OtherActor))
    (bind _asbp_third_person_character (cast `/Game/ThirdPerson/Blueprints/BP_ThirdPersonCharacter` _output_get))
    (set `self.As BP Third Person Character` _asbp_third_person_character)))

(event `self.MonsterTrigger.OnComponentEndOverlap`
  (params (OverlappedComponent :type "PrimitiveComponent Object Reference") (OtherActor :type "Actor Object Reference") (OtherComp :type "PrimitiveComponent Object Reference") (OtherBodyIndex :type Integer))
  (bind _audio (`self.Audio`))
  (if (and (`GameplayStatics.ObjectIsA` OtherActor "/Game/ThirdPerson/Blueprints/BP_ThirdPersonCharacter.BP_ThirdPersonCharacter_C") (not (`self.hasMonsterStarted?`)))
    (`ActorComponent.Activate` _audio true)
    (`AudioComponent.FadeIn` _audio 10.0 1.0 0.0 "Linear")
    (`self.StartMonster`)
    (bind _asgi_store_information (cast `/Game/StopAndBreathe/Blueprints/GI_StoreInformation` (`GameplayStatics.GetGameInstance`)))
    (`/Game/StopAndBreathe/Blueprints/GI_StoreInformation.PlayChaseMusic` _asgi_store_information)))

(event `self.Monster.OnComponentBeginOverlap`
  (params (OverlappedComponent :type "PrimitiveComponent Object Reference") (OtherActor :type "Actor Object Reference") (OtherComp :type "PrimitiveComponent Object Reference") (OtherBodyIndex :type Integer) (bFromSweep :type Boolean) (SweepResult :type "HitResult Structure (by ref)"))
  (if (`GameplayStatics.ObjectIsA` OtherActor "/Game/ThirdPerson/Blueprints/BP_ThirdPersonCharacter.BP_ThirdPersonCharacter_C")
    (set `self.TouchedPlayer` true)
    (`SceneComponent.K2_SetWorldLocation` (`self.Monster`) (`SceneComponent.K2_GetComponentLocation` (`self.Arrow`)) false false)))

(fn `Follow Player`
  (bind (_returnvalue_x _returnvalue_y _returnvalue_z) (`KismetMathLibrary.BreakVector` (`SceneComponent.K2_GetComponentLocation` (`self.Monster`))))
  ;[0.151 0.151 0.151] If true move the monster
  (if (`self.isMonsterTooClose`)
    (set `self.MonsterMoveSpeed` 370.0)
    (else
      (set `self.MonsterMoveSpeed` 200.0)))
  (`SceneComponent.K2_SetWorldLocation` (`self.Monster`) (`KismetMathLibrary.MakeVector` _returnvalue_x (+ _returnvalue_y (* (`self.MonsterMoveSpeed`) (`self.Delta Seconds`))) _returnvalue_z) false false))

(fn `InitialMoveMonsterToPlayer`
  (bind (_returnvalue_x _returnvalue_y _returnvalue_z) (`KismetMathLibrary.BreakVector` (`SceneComponent.K2_GetComponentLocation` (`self.Monster`))))
  (bind (_returnvalue_x_2 _returnvalue_y_2) (`KismetMathLibrary.BreakVector` (`SceneComponent.K2_GetComponentLocation` (`Character.Mesh` (`self.As BP Third Person Character`)))))
  (if (`self.isMonsterTooClose`)
    (`SceneComponent.K2_SetWorldLocation` (`self.Monster`) (`KismetMathLibrary.MakeVector` _returnvalue_x (`KismetMathLibrary.Lerp` (- _returnvalue_y_2 700.0) (`self.StartingMonsterYPos`) (/ (`self.MoveToTimer`) (`self.InitialMoveToTimer`))) _returnvalue_z) false false)
    (else
      (set `self.MoveToTimer` 0.0))))

(fn `isMonsterTooClose`
  (returns (outBool :type Boolean))
  (locals (NewLocalVar :type "Character Object Reference"))
  (bind (_returnvalue_x _returnvalue_y) (`KismetMathLibrary.BreakVector` (`SceneComponent.K2_GetComponentLocation` (`self.Monster`))))
  (bind (_returnvalue_x_2 _returnvalue_y_2) (`KismetMathLibrary.BreakVector` (`SceneComponent.K2_GetComponentLocation` (`Character.Mesh` (`self.As BP Third Person Character`)))))
  (return (not (> _returnvalue_y (- _returnvalue_y_2 (`self.MinMonsterDistanceFromPlayer`))))))

(fn `UserConstructionScript`
  (`MeshComponent.SetScalarParameterValueOnMaterials` (`self.Monster`) "GooJiggleAmount" 50.0))