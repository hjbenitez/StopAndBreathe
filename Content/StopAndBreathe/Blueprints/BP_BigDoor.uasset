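; BP_BigDoor is a double door that opens when every BP_Button linked to it is on.
; On BeginPlay it finds buttons listing it in AttachedObjects and spawns an indicator light mesh for each.
; ActivateInteraction and CancelInteraction refresh the cached button states and update each light's colour and glow.
; The OpenDoors timeline swings both leaves apart with sound once all are on, and reverses when any turns off.
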(event `self.ReceiveBeginPlay`
  (bind (_returnvalue_roll _returnvalue_pitch _returnvalue_yaw) (`KismetMathLibrary.BreakRotator` (`SceneComponent.K2_GetComponentRotation` (`self.rightDoor`))))
  (bind (_returnvalue_location _returnvalue_rotation) (`KismetMathLibrary.BreakTransform` (`SceneComponent.GetRelativeTransform` (`self.Arrow`))))
  (bind (_returnvalue_roll_2 _returnvalue_pitch_2 _returnvalue_yaw_2) (`KismetMathLibrary.BreakRotator` (`SceneComponent.K2_GetComponentRotation` (`self.leftDoor`))))
  (`|ExecutionSequence`
    (:`then_0`
      (set `self.leftStartRot` _returnvalue_yaw_2)
      (set `self.rightStartRot` _returnvalue_yaw)
      (bind _outactors (`GameplayStatics.GetAllActorsOfClass` "/Game/StopAndBreathe/Blueprints/BP_Button.BP_Button_C"))
      (for _array_element _outactors
        (for _array_element_2 (`/Game/StopAndBreathe/Blueprints/BP_Button.AttachedObjects` _array_element)
          (if (== _array_element_2 self)
            (`KismetArrayLibrary.Array_Add` (`self.bookshelvesWithBooks`) _array_element)
            (`KismetArrayLibrary.Array_Add` (`self.bookshelvesFull`) (`/Game/StopAndBreathe/Blueprints/BP_Button.isActive` _array_element))))))
    (:`then_1`
      (for _ (`self.bookshelvesWithBooks`)
        (bind _returnvalue (`AddComponent|NODE_AddStaticMeshComponent-0` :`RelativeTransform` (`KismetMathLibrary.MakeTransform` (+ _returnvalue_location (`self.LightOffset`)) _returnvalue_rotation (0.12 0.0825 0.0825))))
        (`KismetArrayLibrary.Array_Add` (`self.Lights`) _returnvalue)
        (`StaticMeshComponent.SetStaticMesh` _returnvalue "/Engine/EditorMeshes/EditorCube.EditorCube")
        (`PrimitiveComponent.SetMaterial` _returnvalue 0 "/Game/StopAndBreathe/Materials/AssetMaterials/Door/MAT_DoorLight.MAT_DoorLight")
        (set `self.LightOffset` (+ (30.0 0.0 0.0) (`self.LightOffset`)))))))

(event `self.ActivateInteraction`
  (for (_array_element _array_index) (`self.bookshelvesWithBooks`)
    (`KismetArrayLibrary.Array_Set` (`self.bookshelvesFull`) _array_index (`/Game/StopAndBreathe/Blueprints/BP_Button.On` _array_element)))
  (`self.TurnOnLights`)
  (if (not (`KismetArrayLibrary.Array_Contains` (`self.bookshelvesFull`)))
    (`GameplayStatics.PlaySoundAtLocation` "/Game/Audio/MetaSounds/MS_DoorOpenClose.MS_DoorOpenClose" (`KismetMathLibrary.VLerp` (`SceneComponent.K2_GetComponentLocation` (`self.leftDoor`)) (`SceneComponent.K2_GetComponentLocation` (`self.rightDoor`)) 0.5) (struct) 1.0 1.0 0.0 null null null null)
    (bind (_direction _openleft _openright) (`Timeline|OpenDoors` :!label _label)
      (:`Update`
        (`|ExecutionSequence`
          (:`then_0`
            (`SceneComponent.K2_SetWorldRotation` (`self.leftDoor`) (`KismetMathLibrary.MakeRotator` 0.0 0.0 (`KismetMathLibrary.Lerp` (`self.leftStartRot`) (+ (`self.leftStartRot`) (* (`self.openRotation`) -1)) _openleft)) false false))
          (:`then_1`
            (`SceneComponent.K2_SetWorldRotation` (`self.rightDoor`) (`KismetMathLibrary.MakeRotator` 0.0 0.0 (`KismetMathLibrary.Lerp` (`self.rightStartRot`) (+ (`self.rightStartRot`) (`self.openRotation`)) _openright)) false false))))
      (:`Finished`
        (if (`KismetArrayLibrary.Array_Contains` (`self.bookshelvesFull`))
          (set `self.isOpen?` false)
          (else
            (set `self.isOpen?` true)))))))

(event `self.CancelInteraction`
  (for (_array_element _array_index) (`self.bookshelvesWithBooks`)
    (`KismetArrayLibrary.Array_Set` (`self.bookshelvesFull`) _array_index (`/Game/StopAndBreathe/Blueprints/BP_Button.On` _array_element)))
  (if (`KismetArrayLibrary.Array_Contains` (`self.bookshelvesFull`))
    (`self.TurnOffLights`)
    (if (`self.isOpen?`)
      (`GameplayStatics.PlaySoundAtLocation` "/Game/Audio/MetaSounds/MS_DoorOpenClose.MS_DoorOpenClose" (`KismetMathLibrary.VLerp` (`SceneComponent.K2_GetComponentLocation` (`self.leftDoor`)) (`SceneComponent.K2_GetComponentLocation` (`self.rightDoor`)) 0.5) (struct) 1.0 1.0 0.0 null null null null)
      (goto _label :!via `Reverse`)
      (else
        (goto _label :!via `Reverse`)))))

(fn `TurnOffLights`
  (for (_array_element _array_index) (`self.bookshelvesWithBooks`)
    (if (not (`/Game/StopAndBreathe/Blueprints/BP_Button.On` _array_element))
      (bind _output (`|GetArrayItem` (`self.Lights`) _array_index))
      (`MeshComponent.SetVectorParameterValueOnMaterials` _output "Color" (`KismetMathLibrary.Conv_LinearColorToVector` (`self.LightOffColour`)))
      (`MeshComponent.SetScalarParameterValueOnMaterials` _output "EmissiveIntensity" 1.0))))

(fn `TurnOnLights`
  (for (_array_element _array_index) (`self.bookshelvesWithBooks`)
    (if (`/Game/StopAndBreathe/Blueprints/BP_Button.On` _array_element)
      (bind _output (`|GetArrayItem` (`self.Lights`) _array_index))
      (`MeshComponent.SetVectorParameterValueOnMaterials` _output "Color" (`KismetMathLibrary.Conv_LinearColorToVector` (`self.LightOnColour`)))
      (`MeshComponent.SetScalarParameterValueOnMaterials` _output "EmissiveIntensity" 5.0))))

(fn `UserConstructionScript`
  (`|ExecutionSequence`
    (:`then_0`
      (bind _output_get (set `self.DoorArray` (`|MakeArray` (`self.rightDoor`) (`self.leftDoor`))))
      (for _array_element _output_get
        (`KismetArrayLibrary.Array_Add` (`self.DoorStartingScale`) (`SceneComponent.K2_GetComponentScale` _array_element))))))