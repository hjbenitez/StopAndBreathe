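; Trigger volume that zooms the view to a puzzle camera while the player's third-person character stands inside its box.
; On begin overlap, it blends the player controller's view target to the referenced PuzzleCamera.
; On end overlap, it blends back to the character.
; Each switch also passes the active camera component to the character's UpdateCameraRotation.
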(event `self.Box.OnComponentBeginOverlap`
  (params (OverlappedComponent :type "PrimitiveComponent Object Reference") (OtherActor :type "Actor Object Reference") (OtherComp :type "PrimitiveComponent Object Reference") (OtherBodyIndex :type Integer) (bFromSweep :type Boolean) (SweepResult :type "HitResult Structure (by ref)"))
  (bind _puzzlecamera (`self.puzzleCamera`))
  (bind _asbp_third_person_character (cast `/Game/ThirdPerson/Blueprints/BP_ThirdPersonCharacter` OtherActor))
  (bind _asplayer_controller (cast `PlayerController` (`Pawn.GetController` _asbp_third_person_character)))
  (`PlayerController.SetViewTargetWithBlend` _asplayer_controller _puzzlecamera 1.0 "VTBlend_Linear" 0.0 false)
  (`/Game/ThirdPerson/Blueprints/BP_ThirdPersonCharacter.UpdateCameraRotation` _asbp_third_person_character (`CameraActor.CameraComponent` _puzzlecamera)))

(event `self.Box.OnComponentEndOverlap`
  (params (OverlappedComponent :type "PrimitiveComponent Object Reference") (OtherActor :type "Actor Object Reference") (OtherComp :type "PrimitiveComponent Object Reference") (OtherBodyIndex :type Integer))
  (bind _asbp_third_person_character (cast `/Game/ThirdPerson/Blueprints/BP_ThirdPersonCharacter` OtherActor))
  (bind _asplayer_controller (cast `PlayerController` (`Pawn.GetController` _asbp_third_person_character)))
  (`PlayerController.SetViewTargetWithBlend` _asplayer_controller _asbp_third_person_character 1.0 "VTBlend_Linear" 0.0 false)
  (`/Game/ThirdPerson/Blueprints/BP_ThirdPersonCharacter.UpdateCameraRotation` _asbp_third_person_character (`/Game/ThirdPerson/Blueprints/BP_ThirdPersonCharacter.Camera` _asbp_third_person_character)))

(fn `UserConstructionScript`)