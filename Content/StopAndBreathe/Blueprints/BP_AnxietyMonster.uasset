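; BP_AnxietyMonster is a hidden monster that appears and closes in behind the player once they overlap its MonsterTrigger.
; The overlap caches the third-person character, reveals the mesh and starts the chase.
; Tick counts down a timer, printing it, while lerping the monster along world Y toward an offset behind the player, ending early once close enough.
; Normal movement after this initial approach is an empty stub.
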(event `self.ReceiveBeginPlay`
  (`SceneComponent.SetVisibility` (`self.Monster`) false false))

(event `self.ReceiveTick`
  (params (DeltaSeconds :type "Float (single-precision)"))
  (set `self.Delta Seconds` DeltaSeconds)
  (if (and (`self.hasMonsterStarted?`) (> (`self.InitialMoveToTimer`) 0.0))
    (`|ExecutionSequence`
      (:`then_0`
        (bind _output_get (set `self.InitialMoveToTimer` (- (`self.InitialMoveToTimer`) (`self.Delta Seconds`))))
        (`KismetSystemLibrary.PrintString` (`KismetStringLibrary.Conv_DoubleToString` _output_get)))
      (:`then_1`
        (`self.InitialMoveMonsterToPlayer`)))
    (else
      ;[1 1 1] Normal Monster Movement
      (if (`self.hasMonsterStarted?`)
        _))))

(event `self.MonsterTrigger.OnComponentBeginOverlap`
  (params (OverlappedComponent :type "PrimitiveComponent Object Reference") (OtherActor :type "Actor Object Reference") (OtherComp :type "PrimitiveComponent Object Reference") (OtherBodyIndex :type Integer) (bFromSweep :type Boolean) (SweepResult :type "HitResult Structure (by ref)"))
  (bind _output_get (set `self.PlayerCharacter` OtherActor))
  (bind _asbp_third_person_character (cast `/Game/ThirdPerson/Blueprints/BP_ThirdPersonCharacter` _output_get))
  (set `self.As BP Third Person Character` _asbp_third_person_character)
  (`self.StartMonster`))

(event `StartMonster`
  (set `self.hasMonsterStarted?` true)
  (`SceneComponent.SetVisibility` (`self.Monster`) true false))

(fn `InitialMoveMonsterToPlayer`
  (bind (_returnvalue_x _returnvalue_y _returnvalue_z) (`KismetMathLibrary.BreakVector` (`SceneComponent.K2_GetComponentLocation` (`self.Monster`))))
  (bind (_returnvalue_x_2 _returnvalue_y_2) (`KismetMathLibrary.BreakVector` (`SceneComponent.K2_GetComponentLocation` (`Character.Mesh` (`self.As BP Third Person Character`)))))
  (if (not (> _returnvalue_y (- _returnvalue_y_2 550.0)))
    (`SceneComponent.K2_SetWorldLocation` (`self.Monster`) (`KismetMathLibrary.MakeVector` _returnvalue_x (`KismetMathLibrary.Lerp` (- _returnvalue_y_2 500.0) _returnvalue_y (/ (`self.InitialMoveToTimer`) 5.0)) _returnvalue_z) false false)
    (else
      (set `self.InitialMoveToTimer` 0.0))))

(fn `UserConstructionScript`)