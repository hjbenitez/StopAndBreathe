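; Breathing terminal interactable that relays the player's inhale, exhale or off state to its attached objects once activated.
; Overlap radii reveal Niagara control beams and select the terminal, driving its icon widget and beam colours, while Tick spins the fan and tracks balloon platforms.
; Lock input keeps it from switching off when the player leaves.
; Non-red variants cycle a ControlledObject with move input, though state messages still reach every attached object.
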(event `self.ReceiveBeginPlay`
  (`parent.ReceiveBeginPlay`)
  (`|ExecutionSequence`
    (:`then_0`
      (`self.EnableInput` (`GameplayStatics.GetPlayerController` 0)))
    (:`then_1`
      (set `self.ControlledObject` (`|GetArrayItem` (`self.AttachedObjects`))))
    (:`then_2`
      (for _array_element (`self.AttachedObjects`)
        (`self.CreateObjectBeam` _array_element)))
    (:`then_4`
      (`AudioComponent.Play` (`self.Audio`) 0.0))
    (:`then_5`
      (bind _aswb_breathing_terminal_icons (cast `/Game/StopAndBreathe/Blueprints/UI/WB_BreathingTerminalIcons` (`WidgetComponent.GetUserWidgetObject` (`self.InteractWidgetBT`)))
        (:`then`
          (bind _output_get (set `self.IconsPopUI Ref` _aswb_breathing_terminal_icons))
          (set `Widget.Visibility` "Hidden" _output_get)
          (bind _asabp_breathing_terminal (cast `/Game/StopAndBreathe/Blueprints/Interactables/ABP_BreathingTerminal` (`SkeletalMeshComponent.GetAnimInstance` (`self.SkeletalMesh`))))
          (set `self.AnimBlueprintRef` _asabp_breathing_terminal))
        (:`CastFailed`
          (`KismetSystemLibrary.PrintString` "Hello"))))))

(event `self.ReceiveTick`
  (params (DeltaSeconds :type "Float (single-precision)"))
  (bind _controlledobject (`self.ControlledObject`))
  (`parent.ReceiveTick` DeltaSeconds)
  (`|ExecutionSequence`
    (:`then_0`
      (if (`self.isRedCP`)
        (for _array_element (`self.AttachedObjects`)
          (if (`GameplayStatics.ObjectIsA` _array_element "/Game/StopAndBreathe/Blueprints/RedBalloon/BP_RedBalloonPlatformBase.BP_RedBalloonPlatformBase_C")
            (bind _asbp_red_balloon_platform_base (cast `/Game/StopAndBreathe/Blueprints/RedBalloon/BP_RedBalloonPlatformBase` _array_element))
            (`FXSystemComponent.SetVectorParameter` (`BlueprintMapLibrary.Map_Find` (`self.ActorNiagaraMap`) _array_element) "User.EndLoc" (`SceneComponent.K2_GetComponentLocation` (`/Game/StopAndBreathe/Blueprints/RedBalloon/BP_RedBalloonPlatformBase.Platform` _asbp_red_balloon_platform_base)))))
        (elif (`GameplayStatics.ObjectIsA` _controlledobject "/Game/StopAndBreathe/Blueprints/RedBalloon/BP_RedBalloonPlatformBase.BP_RedBalloonPlatformBase_C")
          (bind _asbp_red_balloon_platform_base_2 (cast `/Game/StopAndBreathe/Blueprints/RedBalloon/BP_RedBalloonPlatformBase` _controlledobject))
          (`FXSystemComponent.SetVectorParameter` (`BlueprintMapLibrary.Map_Find` (`self.ActorNiagaraMap`) _controlledobject) "User.EndLoc" (`SceneComponent.K2_GetComponentLocation` (`/Game/StopAndBreathe/Blueprints/RedBalloon/BP_RedBalloonPlatformBase.Platform` _asbp_red_balloon_platform_base_2))))))
    (:`then_1`
      (if (and (`self.isActivate`) (`self.isSelected`))
        (`/Game/StopAndBreathe/Blueprints/UI/WB_BreathingTerminalIcons.UpdateInputStyle` (`self.IconsPopUI Ref`) (`self.ObjectStateController` (`self.Object State`) (`self.isLocked?`)))))
    (:`then_2`
      (if (`self.isActivate`)
        (`self.PlayFanAnim` (`self.ObjectStateController` (`self.Object State`) (`self.isLocked?`)))))))

(event `self.InteractionRadius.OnComponentBeginOverlap`
  (params (OverlappedComponent :type "PrimitiveComponent Object Reference") (OtherActor :type "Actor Object Reference") (OtherComp :type "PrimitiveComponent Object Reference") (OtherBodyIndex :type Integer) (bFromSweep :type Boolean) (SweepResult :type "HitResult Structure (by ref)"))
  (if (and (`GameplayStatics.ObjectIsA` OtherActor "/Game/ThirdPerson/Blueprints/BP_ThirdPersonCharacter.BP_ThirdPersonCharacter_C") (`self.isActivate`))
    (bind _asbp_third_person_character (cast `/Game/ThirdPerson/Blueprints/BP_ThirdPersonCharacter` OtherActor))
    (set `/Game/ThirdPerson/Blueprints/BP_ThirdPersonCharacter.IsInBTRadius` true _asbp_third_person_character)
    (set `self.isSelected` true)
    (set `/Game/ThirdPerson/Blueprints/Blueprint_Components/InteractionComponent.BTinRadius` self (`/Game/ThirdPerson/Blueprints/BP_ThirdPersonCharacter.InteractionComponent` _asbp_third_person_character))
    (`Widget.SetVisibility` (`self.IconsPopUI Ref`) "Visible")
    (`self.ChangeBeamColors` true)))

(event `/Game/StopAndBreathe/Blueprints/Interfaces/BPI_Interactable.InteractableFunction`
  (params (ObjectState :type "/Game/StopAndBreathe/Blueprints/Interactables/ENUM_InteractableStates Enum" :default "NewEnumerator2"))
  (set `self.Object State` ObjectState)
  (if (and (`self.isActivate`) (`self.isSelected`))
    (for _array_element (`self.AttachedObjects`)
      (message `/Game/StopAndBreathe/Blueprints/Interfaces/BPI_Interactable.ObjectFunction` _array_element (`self.ObjectStateController` (`self.Object State`) (`self.isLocked?`))))))

(event `self.InteractionRadius.OnComponentEndOverlap`
  (params (OverlappedComponent :type "PrimitiveComponent Object Reference") (OtherActor :type "Actor Object Reference") (OtherComp :type "PrimitiveComponent Object Reference") (OtherBodyIndex :type Integer))
  (if (and (`GameplayStatics.ObjectIsA` OtherActor "/Game/ThirdPerson/Blueprints/BP_ThirdPersonCharacter.BP_ThirdPersonCharacter_C") (`self.isActivate`))
    (bind _asbp_third_person_character (cast `/Game/ThirdPerson/Blueprints/BP_ThirdPersonCharacter` OtherActor))
    (set `/Game/ThirdPerson/Blueprints/BP_ThirdPersonCharacter.IsInBTRadius` false _asbp_third_person_character)
    (set `self.isSelected` false)
    (set `/Game/ThirdPerson/Blueprints/Blueprint_Components/InteractionComponent.BTinRadius` null (`/Game/ThirdPerson/Blueprints/BP_ThirdPersonCharacter.InteractionComponent` _asbp_third_person_character))
    (if (not (`self.isLocked?`))
      (`Widget.SetVisibility` (`self.IconsPopUI Ref`) "Hidden")
      (`self.ChangeBeamColors` false)
      (bind _output_get (set `self.Object State` "NewEnumerator2"))
      (for _array_element (`self.AttachedObjects`)
        (message `/Game/StopAndBreathe/Blueprints/Interfaces/BPI_Interactable.ObjectFunction` _array_element _output_get))
      (else
        (`Widget.SetVisibility` (`self.IconsPopUI Ref`) "Visible")))))

(event `/Game/StopAndBreathe/Blueprints/Interfaces/BPI_Interactable.CancelInteraction`)

(event `/Game/StopAndBreathe/Blueprints/Interfaces/BPI_Interactable.ActivateInteraction`)

(event `self.PreviewRadius.OnComponentBeginOverlap`
  (params (OverlappedComponent :type "PrimitiveComponent Object Reference") (OtherActor :type "Actor Object Reference") (OtherComp :type "PrimitiveComponent Object Reference") (OtherBodyIndex :type Integer) (bFromSweep :type Boolean) (SweepResult :type "HitResult Structure (by ref)"))
  (if (and (`GameplayStatics.ObjectIsA` OtherActor "/Script/Engine.Character") (`self.isActivate`))
    (`SceneComponent.SetVisibility` (`self.Decal`) true false)
    (for _array_element (`self.ControlBeamsArray`)
      (`ActorComponent.SetActive` _array_element true false))))

(event `EnhancedInput|/Game/ThirdPerson/Input/Actions/IA_Move`
  (params (ActionValue :type "Vector2D Structure") (ElapsedSeconds :type "Float (double-precision)") (TriggeredSeconds :type "Float (double-precision)") (InputAction :type "InputAction Object Reference" :default "/Game/ThirdPerson/Input/Actions/IA_Move.IA_Move"))
  (:`Started`
    (if (and (not (`self.isRedCP`)) (`self.isSelected`))
      (if (> ActionValue_Y 0.0)
        (`self.IncrementArray`)
        (`self.ChangeBeamColors` true)
        (else
          (`self.DecrementArray`)
          (`self.ChangeBeamColors` true))))))

(event `self.PreviewRadius.OnComponentEndOverlap`
  (params (OverlappedComponent :type "PrimitiveComponent Object Reference") (OtherActor :type "Actor Object Reference") (OtherComp :type "PrimitiveComponent Object Reference") (OtherBodyIndex :type Integer))
  (if (and (`GameplayStatics.ObjectIsA` OtherActor "/Script/Engine.Character") (`self.isActivate`))
    (`SceneComponent.SetVisibility` (`self.Decal`) false false)
    (for _array_element (`self.ControlBeamsArray`)
      (`ActorComponent.SetActive` _array_element false false))))

(event `/Game/StopAndBreathe/Blueprints/Interfaces/BPI_Interactable.ActivateObject`
  (`parent.ActivateObject`)
  (`AudioComponent.Stop` (`self.Audio`))
  (for (_array_element _array_index) (`self.TrueMats`)
    (`PrimitiveComponent.SetMaterial` (`self.SkeletalMesh`) _array_index _array_element)))

(event `/Game/StopAndBreathe/Blueprints/Interfaces/BPI_Interactable.ActivateButtonPrompt`)

(event `/Game/StopAndBreathe/Blueprints/Interfaces/BPI_Interactable.DeactivateButtonPrompt`)

(event `/Game/StopAndBreathe/Blueprints/Interfaces/BPI_Interactable.DeactivateObject`
  (`parent.DeactivateObject`))

(event `EnhancedInput|/Game/ThirdPerson/Input/Actions/IA_Lock`
  (params (ActionValue :type Boolean) (ElapsedSeconds :type "Float (double-precision)") (TriggeredSeconds :type "Float (double-precision)") (InputAction :type "InputAction Object Reference" :default "/Game/ThirdPerson/Input/Actions/IA_Lock.IA_Lock"))
  (:`Started`
    (if (`self.isSelected`)
      (if (`self.isLocked?`)
        (bind _output_get (set `self.isLocked?` false))
        (`/Game/StopAndBreathe/Blueprints/UI/WB_BreathingTerminalIcons.SetLock` (`self.IconsPopUI Ref`) _output_get)
        (for _array_element (`self.AttachedObjects`)
          (message `/Game/StopAndBreathe/Blueprints/Interfaces/BPI_Interactable.ObjectFunction` _array_element "NewEnumerator2"))
        (else
          (bind _output_get_2 (set `self.isLocked?` true))
          (`/Game/StopAndBreathe/Blueprints/UI/WB_BreathingTerminalIcons.SetLock` (`self.IconsPopUI Ref`) _output_get_2))))))

(fn `ChangeBeamColors`
  (params (isSettingToControlColor :type Boolean))
  (for _array_element (`self.ControlBeamsArray`)
    (`NiagaraComponent.SetVariableLinearColor` _array_element "User.Linear Color" (`self.NotControlColor`)))
  (if isSettingToControlColor
    (for _array_element_2 (`self.ControlBeamsArray`)
      (`NiagaraComponent.SetVariableLinearColor` _array_element_2 "User.Linear Color" (`self.ControlColor`)))))

(fn `CreateObjectBeam`
  (params (InActor :type "Actor Object Reference"))
  (bind _returnvalue (`NiagaraFunctionLibrary.SpawnSystemAttached` "/Game/StopAndBreathe/Materials/ParticleSystems/P_ControlBeam2.P_ControlBeam2" (`self.Arrow`) "None" (0.0 0.0 0.0) (struct) "KeepRelativeOffset"))
  (`BlueprintMapLibrary.Map_Add` (`self.ActorNiagaraMap`) InActor _returnvalue)
  (`KismetArrayLibrary.Array_Add` (`self.ControlBeamsArray`) _returnvalue)
  (`FXSystemComponent.SetVectorParameter` _returnvalue "User.EndLoc" (`self.K2_GetActorLocation` InActor))
  (`ActorComponent.SetActive` _returnvalue false false)
  (`NiagaraComponent.SetVariableLinearColor` _returnvalue "User.Linear Color" (`self.NotControlColor`)))

(fn `DecrementArray`
  (bind _posinarray (`self.PosInArray`))
  (`/Engine/EditorBlueprintResources/StandardMacros.DecrementInt` (`self.PosInArray`)
    (:`  `
      (if (< (`self.PosInArray`) 0)
        (set `self.PosInArray` 0))
      (bind _output_get (set `self.ControlledObject` (`|GetArrayItem` (`self.AttachedObjects`) _posinarray)))
      (`KismetSystemLibrary.PrintString` (`KismetStringLibrary.Concat_StrStr` (`KismetStringLibrary.Conv_IntToString` _posinarray) (`KismetSystemLibrary.GetDisplayName` _output_get))))))

(fn `IncrementArray`
  (returns (ControlledObject :type "Actor Object Reference"))
  (bind _result (`/Engine/EditorBlueprintResources/StandardMacros.IncrementInt` (`self.PosInArray`))
    (:`  `
      (if (> (`self.PosInArray`) (- (`KismetArrayLibrary.Array_Length` (`self.AttachedObjects`)) 1))
        (set `self.PosInArray` (- (`KismetArrayLibrary.Array_Length` (`self.AttachedObjects`)) 1)))
      (bind _output_get (set `self.ControlledObject` (`|GetArrayItem` (`self.AttachedObjects`) (`self.PosInArray`))))
      (return _output_get))))

(fn `ObjectStateController`
  (params (InState :type "/Game/StopAndBreathe/Blueprints/Interactables/ENUM_InteractableStates Enum" :default "NewEnumerator2") (`isLocked?` :type Boolean))
  (returns (outState :type "/Game/StopAndBreathe/Blueprints/Interactables/ENUM_InteractableStates Enum"))
  (locals (L_InObjectState :type "/Game/StopAndBreathe/Blueprints/Interactables/ENUM_InteractableStates Enum" :default "NewEnumerator2") (L_LockedState :type "/Game/StopAndBreathe/Blueprints/Interactables/ENUM_InteractableStates Enum" :default "NewEnumerator2"))
  (set `local.L_InObjectState` InState)
  (if `isLocked?`
    (switch `/Game/StopAndBreathe/Blueprints/Interactables/ENUM_InteractableStates` (`local.L_InObjectState`)
      (:`NewEnumerator0`
        (bind _output_get (set `local.L_InObjectState` "NewEnumerator0"))
        (set `local.L_LockedState` _output_get))
      (:`NewEnumerator1`
        (bind _output_get_2 (set `local.L_InObjectState` "NewEnumerator1"))
        (set `local.L_LockedState` _output_get_2)))
    (return (`local.L_LockedState`))
    (else
      (return (`local.L_InObjectState`)))))

(fn `PlayFanAnim`
  (params (InState :type "/Game/StopAndBreathe/Blueprints/Interactables/ENUM_InteractableStates Enum" :default "NewEnumerator2"))
  (switch `/Game/StopAndBreathe/Blueprints/Interactables/ENUM_InteractableStates` InState
    (:`NewEnumerator2`
      (bind _output_get (set `self.Rotation` (+ (`self.Rotation`) 0.0)))
      (`/Game/StopAndBreathe/Blueprints/Interactables/ABP_BreathingTerminal.Rotation Event` (`self.AnimBlueprintRef`) _output_get))
    (:`NewEnumerator0`
      (bind _output_get_2 (set `self.Rotation` (+ (`self.Rotation`) 2.0)))
      (`/Game/StopAndBreathe/Blueprints/Interactables/ABP_BreathingTerminal.Rotation Event` (`self.AnimBlueprintRef`) _output_get_2))
    (:`NewEnumerator1`
      (bind _output_get_3 (set `self.Rotation` (- (`self.Rotation`) 2.0)))
      (`/Game/StopAndBreathe/Blueprints/Interactables/ABP_BreathingTerminal.Rotation Event` (`self.AnimBlueprintRef`) _output_get_3))))

(fn `UserConstructionScript`
  (`parent.UserConstructionScript`)
  (`|ExecutionSequence`
    (:`then_0`
      (if (`self.isRedCP`)
        (`PrimitiveComponent.SetMaterial` (`self.SkeletalMesh`) 0 "/Game/StopAndBreathe/Materials/AssetMaterials/BreathingTerminal/MAT_BreathingTerminalBase_Red.MAT_BreathingTerminalBase_Red")
        (`PrimitiveComponent.SetMaterial` (`self.SkeletalMesh`) 1 "/Game/StopAndBreathe/Materials/AssetMaterials/BreathingTerminal/RedBreathingTerminalFan.RedBreathingTerminalFan")
        (set `self.TrueMats` (`MeshComponent.GetMaterials` (`self.SkeletalMesh`)))
        (else
          (`PrimitiveComponent.SetMaterial` (`self.SkeletalMesh`) 0 "/Game/StopAndBreathe/Materials/AssetMaterials/BreathingTerminal/BreathingTerminalBase_Blue.BreathingTerminalBase_Blue")
          (`PrimitiveComponent.SetMaterial` (`self.SkeletalMesh`) 1 "/Game/StopAndBreathe/Materials/Development/Blue_Mat.Blue_Mat")
          (set `self.TrueMats` (`MeshComponent.GetMaterials` (`self.SkeletalMesh`))))))
    (:`then_1`
      (`PrimitiveComponent.SetMaterial` (`self.SkeletalMesh`) 0 "/Game/StopAndBreathe/Materials/Shaders/BAOBlocker.BAOBlocker")
      (`PrimitiveComponent.SetMaterial` (`self.SkeletalMesh`) 1 "/Game/StopAndBreathe/Materials/Shaders/BAOBlocker.BAOBlocker"))))