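; Pickable book box that the player carries and places on shelves (BP_Button) matching its book type, or on snap points.
; Pickup eases it to the character's arrow and physics-constrains it to their mesh.
; A box trace blocks release inside walls except at matching shelves; valid release breaks the constraint and may snap it.
; It starts frozen with a blocker material until activated, and also handles prompts, impact sounds and out-of-bounds resets.
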(event `self.ReceiveBeginPlay`
  (`parent.ReceiveBeginPlay`)
  (`|ExecutionSequence`
    (:`then_0`
      (set `self.BeginningTransform` (`SceneComponent.K2_GetComponentToWorld` (`self.StaticMesh`))))
    (:`then_1`
      (`PrimitiveComponent.SetSimulatePhysics` (`self.StaticMesh`) false)
      (if (not (`self.noPlaySound`))
        (`AudioComponent.Play` (`self.Audio`) 0.0)))
    (:`then_2`
      (bind _aswb_interaction_prompt (cast `/Game/StopAndBreathe/Blueprints/UI/WB_InteractionPrompt` (`WidgetComponent.GetUserWidgetObject` (`self.InteractWidget`))))
      (set `self.As WB Interaction Prompt_0` _aswb_interaction_prompt))
    (:`then_3`
      (`PrimitiveComponent.SetMaterial` (`self.StaticMesh`) 0 (`self.BAOBlocker`)))))

(event `/Game/StopAndBreathe/Blueprints/Interfaces/BPI_Interactable.ActivateInteraction`
  (`parent.ActivateInteraction`)
  ;[1 1 1] Move object to desired position then constain box to player
  (if (`self.isActivate`)
    (`PrimitiveComponent.SetSimulatePhysics` (`self.StaticMesh`) true)
    (`PrimitiveComponent.SetCollisionResponseToChannel` (`self.StaticMesh`) "ECC_Pawn" "ECR_Ignore")
    (bind _asbp_third_person_character (cast `/Game/ThirdPerson/Blueprints/BP_ThirdPersonCharacter` (`.ReturnValue` (`GameplayStatics.FindNearestActor` (0.0 0.0 0.0) (`PrimitiveComponent.GetOverlappingActors` (`self.InteractionRadius`) "/Game/ThirdPerson/Blueprints/BP_ThirdPersonCharacter.BP_ThirdPersonCharacter_C")))))
    (bind _output_get (set `self.BP Third Person Character` _asbp_third_person_character))
    (bind (_returnvalue_location _returnvalue_rotation) (`KismetMathLibrary.BreakTransform` (`SceneComponent.K2_GetComponentToWorld` (`/Game/ThirdPerson/Blueprints/BP_ThirdPersonCharacter.Arrow_Box` _output_get))))
    (`KismetSystemLibrary.MoveComponentTo` (`self.StaticMesh`) _returnvalue_location _returnvalue_rotation true true 0.1 true)
    (`PhysicsConstraintComponent.SetConstrainedComponents` (`self.PhysicsConstraint`) (`self.StaticMesh`) "None" (`Character.Mesh` (`self.BP Third Person Character`)) "None")
    (set `self.IsBeingHeld` true)))

(event `/Game/StopAndBreathe/Blueprints/Interfaces/BPI_Interactable.CancelInteraction`
  (bind (_boxsnaplocation _boxsnaprotation _shouldsnaptoposition) (`self.SnapPosition`))
  (if (`self.isActivate`)
    (if (and (`self.CheckIfCubeIsInWall`) (not (`self.isMatchingShelf` (`PrimitiveComponent.GetOverlappingActors` (`self.StaticMesh`) "/Game/StopAndBreathe/Blueprints/BP_Button.BP_Button_C"))))
      (set `/Game/ThirdPerson/Blueprints/BP_ThirdPersonCharacter.isInteracting` true (`self.BP Third Person Character`))
      (else
        (set `/Game/ThirdPerson/Blueprints/Blueprint_Components/InteractionComponent.ActivatedInteractable` null (`/Game/ThirdPerson/Blueprints/BP_ThirdPersonCharacter.InteractionComponent` (`self.BP Third Person Character`)))
        ;[1 1 1] Break Connection then reenable player collisions
        (`PhysicsConstraintComponent.BreakConstraint` (`self.PhysicsConstraint`))
        (`KismetSystemLibrary.Delay` 0.01)
        (`PrimitiveComponent.SetCollisionResponseToChannel` (`self.StaticMesh`) "ECC_Pawn" "ECR_Block")
        (set `self.IsBeingHeld` false)
        ;[1 1 1] Check if box in the the snap point radius, then snap to point
        (if _shouldsnaptoposition
          (`KismetSystemLibrary.MoveComponentTo` (`self.StaticMesh`) _boxsnaplocation _boxsnaprotation true true 0.4)
          (`PrimitiveComponent.SetSimulatePhysics` (`self.StaticMesh`) false))))))

(event `self.ReceiveTick`
  (params (DeltaSeconds :type "Float (single-precision)"))
  (bind _isbeingheld (`self.IsBeingHeld`))
  (bind (_returnvalue_x _returnvalue_y _returnvalue_z) (`KismetMathLibrary.BreakVector` (`SceneComponent.K2_GetComponentLocation` (`self.BoxCenter`))))
  (`parent.ReceiveTick` DeltaSeconds)
  (`|ExecutionSequence`
    (:`then_0`
      ;[1 1 1] Check if box is inside object, then show blocker icon
      (`KismetSystemLibrary.Delay` 0.2)
      (if _isbeingheld
        (if (and _isbeingheld (`self.CheckIfCubeIsInWall`) (not (`self.isMatchingShelf` (`PrimitiveComponent.GetOverlappingActors` (`self.StaticMesh`) "/Game/StopAndBreathe/Blueprints/BP_Button.BP_Button_C"))))
          (`/Game/StopAndBreathe/Blueprints/UI/WB_InteractionPrompt.ShowBlock` (`self.As WB Interaction Prompt_0`))
          (else
            (`/Game/StopAndBreathe/Blueprints/UI/WB_InteractionPrompt.RemoveBlock` (`self.As WB Interaction Prompt_0`))))))
    (:`then_1`
      ;[1 1 1] Set Interact Prompt to be always above box in the game world
      (if (and (`self.isActivate`) (`self.isPlayerInProximity`))
        (`SceneComponent.K2_SetWorldLocation` (`self.InteractWidget`) (`KismetMathLibrary.MakeVector` _returnvalue_x _returnvalue_y (+ _returnvalue_z 60.0)) false false)))
    (:`then_2`
      (if (`self.IsBeingHeld`)
        (`self.ActivateButtonPrompt`)))
    (:`then_3`
      (`self.PromptTextHandler`))))

(event `/Game/StopAndBreathe/Blueprints/Interfaces/BPI_OutOfBounds.OutOfBounds`
  (bind _beginningtransform_location (`KismetMathLibrary.BreakTransform` (`self.BeginningTransform`)))
  ;[1 1 1] Out of Bounds Reset
  (`KismetSystemLibrary.Delay` 0.2)
  (`SceneComponent.K2_SetWorldLocation` (`self.StaticMesh`) _beginningtransform_location false true))

(event `/Game/StopAndBreathe/Blueprints/Interfaces/BPI_Interactable.ActivateObject`
  ;[1 1 1] Remove Anxiety Stuff
  (`parent.ActivateObject`)
  (`PrimitiveComponent.SetSimulatePhysics` (`self.StaticMesh`) true)
  (`AudioComponent.Stop` (`self.Audio`))
  (`PrimitiveComponent.SetMaterial` (`self.StaticMesh`) 0 (`self.TrueMat`)))

(event `/Game/StopAndBreathe/Blueprints/Interfaces/BPI_Interactable.DeactivateObject`
  (`parent.DeactivateObject`)
  (`PrimitiveComponent.SetSimulatePhysics` (`self.StaticMesh`) false))

(event `self.ReceiveHit`
  (params (MyComp :type "PrimitiveComponent Object Reference") (Other :type "Actor Object Reference") (OtherComp :type "PrimitiveComponent Object Reference") (bSelfMoved :type Boolean) (HitLocation :type "Vector Structure") (HitNormal :type "Vector Structure") (NormalImpulse :type "Vector Structure") (Hit :type "HitResult Structure (by ref)"))
  ;[1 1 1] Impact Sound
  (if (> (`KismetMathLibrary.VSize` (`SceneComponent.GetComponentVelocity` MyComp)) 100.0)
    (`GameplayStatics.PlaySoundAtLocation` "/Game/Audio/MetaSounds/MS_BookImpact.MS_BookImpact" HitLocation (struct) 1.0 1.0 0.0 null null null null)))

(fn `CheckIfCubeIsInWall`
  (returns (OutBool :type Boolean))
  (locals (bCubeInWall :type Boolean) (NewLocalVar :type "PrimitiveComponent Object Reference") (NewLocalVar_0 :type "Array of HitResult Structure"))
  (bind _staticmesh (`self.StaticMesh`))
  (bind (_returnvalue_x _returnvalue_y _returnvalue_z) (`KismetMathLibrary.BreakVector` (`SceneComponent.K2_GetComponentLocation` _staticmesh)))
  (bind _returnvalue (`KismetMathLibrary.MakeVector` _returnvalue_x _returnvalue_y (+ _returnvalue_z 35.0)))
  (bind _outhits (`KismetSystemLibrary.BoxTraceMultiForObjects` :`Start` _returnvalue :`End` _returnvalue :`HalfSize` (32.5 32.5 35.0) :`Orientation` (`SceneComponent.K2_GetComponentRotation` _staticmesh) :`ObjectTypes` (`|MakeArray` "ObjectTypeQuery1" :!type "EObjectTypeQuery Enum") :`DrawTime` 0.5))
  (return (`KismetArrayLibrary.Array_IsNotEmpty` _outhits)))

(fn `isMatchingShelf`
  (params (OverlappingBoxes :type "Array of Actor Object Reference"))
  (returns (ReturnValue :type Boolean))
  (bind _asbp_button (cast `/Game/StopAndBreathe/Blueprints/BP_Button` (`.ReturnValue` (`GameplayStatics.FindNearestActor` (`SceneComponent.K2_GetComponentLocation` (`self.StaticMesh`)) OverlappingBoxes))))
  (bind _booktype (`/Game/StopAndBreathe/Blueprints/BP_Button.BookType` _asbp_button))
  (return (or (`|EnumEquality` (`self.BookType`) _booktype) (`|EnumEquality` _booktype "NewEnumerator4"))))

(fn `PromptTextHandler`
  (locals (OverlappingButtons :type "Array of Actor Object Reference"))
  (bind _overlappingactors (`PrimitiveComponent.GetOverlappingActors` (`self.StaticMesh`) "/Game/StopAndBreathe/Blueprints/BP_Button.BP_Button_C"))
  (set `local.OverlappingButtons` _overlappingactors)
  (if (and (or (`KismetArrayLibrary.Array_IsNotEmpty` _overlappingactors) (`KismetArrayLibrary.Array_IsNotEmpty` (`PrimitiveComponent.GetOverlappingActors` (`self.StaticMesh`) "/Game/StopAndBreathe/Blueprints/BP_SnapPoint.BP_SnapPoint_C"))) (`self.IsBeingHeld`))
    (if (`self.isMatchingShelf` (`local.OverlappingButtons`))
      (`TextBlock.SetText` (`/Game/StopAndBreathe/Blueprints/UI/WB_InteractionPrompt.TextBlock_189` (`self.As WB Interaction Prompt_0`)) "Place"))
    (elif (`self.IsBeingHeld`)
      (`TextBlock.SetText` (`/Game/StopAndBreathe/Blueprints/UI/WB_InteractionPrompt.TextBlock_189` (`self.As WB Interaction Prompt_0`)) "Drop")
      (else
        (`TextBlock.SetText` (`/Game/StopAndBreathe/Blueprints/UI/WB_InteractionPrompt.TextBlock_189` (`self.As WB Interaction Prompt_0`)) "Pick Up")))))

(fn `SnapPosition`
  (returns (BoxSnapLocation :type "Vector Structure") (BoxSnapRotation :type "Rotator Structure") (ShouldSnapToPosition :type Boolean))
  (locals (L_ShouldSnapToPosition :type Boolean) (L_BoxSnapRotation :type "Rotator Structure" :default (struct)) (L_BoxSnapLocation :type "Vector Structure" :default (0.0 0.0 0.0)))
  (bind _staticmesh (`self.StaticMesh`))
  (bind _staticmesh_2 (`self.StaticMesh`))
  (bind _overlappingactors (`PrimitiveComponent.GetOverlappingActors` _staticmesh "/Game/StopAndBreathe/Blueprints/BP_Button.BP_Button_C"))
  (bind _overlappingactors_2 (`PrimitiveComponent.GetOverlappingActors` _staticmesh_2 "/Game/StopAndBreathe/Blueprints/BP_SnapPoint.BP_SnapPoint_C"))
  (if (`KismetArrayLibrary.Array_IsNotEmpty` _overlappingactors)
    (bind _asbp_button (cast `/Game/StopAndBreathe/Blueprints/BP_Button` (`.ReturnValue` (`GameplayStatics.FindNearestActor` (`SceneComponent.K2_GetComponentLocation` _staticmesh) _overlappingactors))))
    (set `local.L_ShouldSnapToPosition` (`self.isMatchingShelf` _overlappingactors))
    (bind (_returnvalue_location _returnvalue_rotation) (`KismetMathLibrary.BreakTransform` (`SceneComponent.K2_GetComponentToWorld` (`/Game/StopAndBreathe/Blueprints/BP_Button.BoxSnapPoint` _asbp_button))))
    (set `local.L_BoxSnapLocation` _returnvalue_location)
    (set `local.L_BoxSnapRotation` _returnvalue_rotation)
    (elif (`KismetArrayLibrary.Array_IsNotEmpty` _overlappingactors_2)
      (bind _asbp_snap_point (cast `/Game/StopAndBreathe/Blueprints/BP_SnapPoint` (`.ReturnValue` (`GameplayStatics.FindNearestActor` (`SceneComponent.K2_GetComponentLocation` _staticmesh_2) _overlappingactors_2))))
      (set `local.L_ShouldSnapToPosition` true)
      (bind (_returnvalue_location_2 _returnvalue_rotation_2) (`KismetMathLibrary.BreakTransform` (`SceneComponent.K2_GetComponentToWorld` (`/Game/StopAndBreathe/Blueprints/BP_SnapPoint.SnapPoint` _asbp_snap_point))))
      (set `local.L_BoxSnapLocation` _returnvalue_location_2)
      (set `local.L_BoxSnapRotation` _returnvalue_rotation_2)
      (else
        (set `local.L_ShouldSnapToPosition` false))))
  (return (`local.L_BoxSnapLocation`) (`local.L_BoxSnapRotation`) (`local.L_ShouldSnapToPosition`)))

(fn `UserConstructionScript`
  (`parent.UserConstructionScript`)
  (`|ExecutionSequence`
    (:`then_0`
      (set `self.TrueMat` (`|GetArrayItem` (`self.BookMaterials`) (`KismetMathLibrary.Conv_ByteToInt` (`self.BookType`)))))
    (:`then_1`
      (`PrimitiveComponent.SetMaterial` (`self.StaticMesh`) 0 (`self.TrueMat`)))))