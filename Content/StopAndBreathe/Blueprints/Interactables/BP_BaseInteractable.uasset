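; Base interactable Blueprint that manages a button prompt widget and a player-proximity flag for interactable objects.
; ActivateObject sets IsActivate, which gates showing the prompt through ActivateButtonPrompt and hiding it when the third-person character leaves InteractionRadius.
; ActivateInteraction and CancelInteraction switch the prompt text between "Confirm" and "Interact".
; Begin overlap and DeactivateObject are empty, so showing the prompt relies on ActivateButtonPrompt being called.
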(event `self.ReceiveBeginPlay`)

(event `/Game/StopAndBreathe/Blueprints/Interfaces/BPI_Interactable.ActivateButtonPrompt`
  (if (`self.isActivate`)
    (`SceneComponent.SetVisibility` (`self.InteractWidget`) true false)
    (set `self.isPlayerInProximity` true)))

(event `self.InteractionRadius.OnComponentBeginOverlap`
  (params (OverlappedComponent :type "PrimitiveComponent Object Reference") (OtherActor :type "Actor Object Reference") (OtherComp :type "PrimitiveComponent Object Reference") (OtherBodyIndex :type Integer) (bFromSweep :type Boolean) (SweepResult :type "HitResult Structure (by ref)")))

(event `/Game/StopAndBreathe/Blueprints/Interfaces/BPI_Interactable.DeactivateButtonPrompt`
  (`SceneComponent.SetVisibility` (`self.InteractWidget`) false false :!label _label)
  (set `self.isPlayerInProximity` false))

(event `/Game/StopAndBreathe/Blueprints/Interfaces/BPI_Interactable.ActivateInteraction`
  (bind _aswb_interaction_prompt (cast `/Game/StopAndBreathe/Blueprints/UI/WB_InteractionPrompt` (`WidgetComponent.GetUserWidgetObject` (`self.InteractWidget`))))
  (`TextBlock.SetText` (`/Game/StopAndBreathe/Blueprints/UI/WB_InteractionPrompt.TextBlock_189` _aswb_interaction_prompt) "Confirm"))

(event `self.InteractionRadius.OnComponentEndOverlap`
  (params (OverlappedComponent :type "PrimitiveComponent Object Reference") (OtherActor :type "Actor Object Reference") (OtherComp :type "PrimitiveComponent Object Reference") (OtherBodyIndex :type Integer))
  (if (and (`GameplayStatics.ObjectIsA` OtherActor "/Game/ThirdPerson/Blueprints/BP_ThirdPersonCharacter.BP_ThirdPersonCharacter_C") (`self.isActivate`))
    (goto _label)))

(event `/Game/StopAndBreathe/Blueprints/Interfaces/BPI_Interactable.CancelInteraction`
  (bind _aswb_interaction_prompt (cast `/Game/StopAndBreathe/Blueprints/UI/WB_InteractionPrompt` (`WidgetComponent.GetUserWidgetObject` (`self.InteractWidget`))))
  (`TextBlock.SetText` (`/Game/StopAndBreathe/Blueprints/UI/WB_InteractionPrompt.TextBlock_189` _aswb_interaction_prompt) "Interact"))

(event `/Game/StopAndBreathe/Blueprints/Interfaces/BPI_Interactable.ActivateObject`
  (set `self.isActivate` true))

(event `/Game/StopAndBreathe/Blueprints/Interfaces/BPI_Interactable.DeactivateObject`)

(fn `UserConstructionScript`)