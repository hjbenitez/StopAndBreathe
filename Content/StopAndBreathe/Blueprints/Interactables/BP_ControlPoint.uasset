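; Breathing terminal interactable that relays inhale/exhale/off states to its attached objects and plays a matching fan animation.
; Red terminals drive all attached objects at once, while blue ones drive one, cycled with IA_Move while selected.
; Niagara beams link each object, appear on character overlap, recolor to show control and track moving balloon platforms on Tick.
; It starts goo-covered with looping animation and audio until ActivateObject restores its materials.
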(event `self.ReceiveBeginPlay`
  (`parent.ReceiveBeginPlay`)
  (`|ExecutionSequence`
    (:`then_0`
      (`self.EnableInput` (`GameplayStatics.GetPlayerController` 0)))
    (:`then_1`
      (set `self.ControlledObject` (`|GetArrayItem` (`self.AttachedObjects`))))
    (:`then_2`
      (for _array_element (`self.AttachedObjects`)
        (`self.CreateObjectBeam` _array_element)))
    (:`then_3`
      (bind _returnvalue (`|CreateWidget` "/Game/StopAndBreathe/Blueprints/UI/WB_BreathingTerminalIcons.WB_BreathingTerminalIcons_C" (`GameplayStatics.GetPlayerController` 0)))
      (set `self.InputWidget` _returnvalue))
    (:`then_4`
      (`AudioComponent.Play` (`self.Audio`) 0.0)
      (`PrimitiveComponent.SetMaterial` (`self.SkeletalMesh`) 0 "/Game/StopAndBreathe/Materials/Shaders/Goo.Goo")
      (`PrimitiveComponent.SetMaterial` (`self.SkeletalMesh`) 1 "/Game/StopAndBreathe/Materials/Shaders/Goo.Goo")
      (`SkeletalMeshComponent.PlayAnimation` (`self.SkeletalMesh`) null true))))

(event `self.ReceiveTick`
  (params (DeltaSeconds :type "Float (single-precision)"))
  (bind _controlledobject (`self.ControlledObject`))
  (`parent.ReceiveTick` DeltaSeconds)
  (if (`self.isRedCP`)
    (for _array_element (`self.AttachedObjects`)
      (if (`GameplayStatics.ObjectIsA` _array_element "/Game/StopAndBreathe/Blueprints/RedBalloon/BP_RedBalloonPlatformBase.BP_RedBalloonPlatformBase_C")
        (bind _asbp_red_balloon_platform_base (cast `/Game/StopAndBreathe/Blueprints/RedBalloon/BP_RedBalloonPlatformBase` _array_element))
        (`FXSystemComponent.SetVectorParameter` (`BlueprintMapLibrary.Map_Find` (`self.ActorNiagaraMap`) _array_element) "User.EndLoc" (`SceneComponent.K2_GetComponentLocation` (`/Game/StopAndBreathe/Blueprints/RedBalloon/BP_RedBalloonPlatformBase.Platform` _asbp_red_balloon_platform_base)))))
    (elif (`GameplayStatics.ObjectIsA` _controlledobject "/Game/StopAndBreathe/Blueprints/RedBalloon/BP_RedBalloonPlatformBase.BP_RedBalloonPlatformBase_C")
      (bind _asbp_red_balloon_platform_base_2 (cast `/Game/StopAndBreathe/Blueprints/RedBalloon/BP_RedBalloonPlatformBase` _controlledobject))
      (`FXSystemComponent.SetVectorParameter` (`BlueprintMapLibrary.Map_Find` (`self.ActorNiagaraMap`) _controlledobject) "User.EndLoc" (`SceneComponent.K2_GetComponentLocation` (`/Game/StopAndBreathe/Blueprints/RedBalloon/BP_RedBalloonPlatformBase.Platform` _asbp_red_balloon_platform_base_2))))))

(event `self.Sphere.OnComponentBeginOverlap`
  (params (OverlappedComponent :type "PrimitiveComponent Object Reference") (OtherActor :type "Actor Object Reference") (OtherComp :type "PrimitiveComponent Object Reference") (OtherBodyIndex :type Integer) (bFromSweep :type Boolean) (SweepResult :type "HitResult Structure (by ref)"))
  (if (and (`GameplayStatics.ObjectIsA` OtherActor "/Script/Engine.Character") (`self.isActivate`))
    (for _array_element (`self.ControlBeamsArray`)
      (`ActorComponent.SetActive` _array_element true false))))

(event `/Game/StopAndBreathe/Blueprints/Interfaces/BPI_Interactable.InteractableFunction`
  (params (ObjectState :type "/Game/StopAndBreathe/Blueprints/Interactables/ENUM_InteractableStates Enum" :default "NewEnumerator2"))
  (if (and (`self.isActivate`) (`self.isSelected`))
    (if (`self.isRedCP`)
      (for _array_element (`self.AttachedObjects`)
        (message `/Game/StopAndBreathe/Blueprints/Interfaces/BPI_Interactable.ObjectFunction` _array_element ObjectState)
        (`self.PlayFanAnim` ObjectState))
      (else
        (message `/Game/StopAndBreathe/Blueprints/Interfaces/BPI_Interactable.ObjectFunction` (`self.ControlledObject`) ObjectState)
        (`self.PlayFanAnim` ObjectState)))))

(event `self.Sphere.OnComponentEndOverlap`
  (params (OverlappedComponent :type "PrimitiveComponent Object Reference") (OtherActor :type "Actor Object Reference") (OtherComp :type "PrimitiveComponent Object Reference") (OtherBodyIndex :type Integer))
  (if (and (`GameplayStatics.ObjectIsA` OtherActor "/Script/Engine.Character") (`self.isActivate`))
    (for _array_element (`self.ControlBeamsArray`)
      (`ActorComponent.SetActive` _array_element false false))))

(event `/Game/StopAndBreathe/Blueprints/Interfaces/BPI_Interactable.CancelInteraction`
  (`parent.CancelInteraction`)
  (if (`self.isActivate`)
    (set `self.isSelected` false)
    (`self.ChangeBeamColors` false)
    (`Widget.RemoveFromParent` (`self.InputWidget`))))

(event `/Game/StopAndBreathe/Blueprints/Interfaces/BPI_Interactable.ActivateInteraction`
  (`parent.ActivateInteraction`)
  (if (`self.isActivate`)
    (set `self.isSelected` true)
    (`UserWidget.AddToViewport` (`self.InputWidget`) 0)
    (if (`self.isRedCP`)
      (if true
        (for _array_element (`self.ControlBeamsArray`)
          (`NiagaraComponent.SetVariableLinearColor` _array_element "User.Linear Color" (`self.ControlColor`))))
      (else
        (`self.ChangeBeamColors` true)))))

(event `/Game/StopAndBreathe/Blueprints/Interfaces/BPI_Interactable.ActivateObject`
  (`parent.ActivateObject`)
  (`AudioComponent.Stop` (`self.Audio`))
  (for (_array_element _array_index) (`self.StartingMats`)
    (`PrimitiveComponent.SetMaterial` (`self.SkeletalMesh`) _array_index _array_element)
    (`SkeletalMeshComponent.Play` (`self.SkeletalMesh`) true)))

(event `/Game/StopAndBreathe/Blueprints/Interfaces/BPI_Interactable.DeactivateObject`
  (`parent.DeactivateObject`))

(event `EnhancedInput|/Game/ThirdPerson/Input/Actions/IA_Move`
  (params (ActionValue :type "Vector2D Structure") (ElapsedSeconds :type "Float (double-precision)") (TriggeredSeconds :type "Float (double-precision)") (InputAction :type "InputAction Object Reference" :default "/Game/ThirdPerson/Input/Actions/IA_Move.IA_Move"))
  (:`Started`
    (if (and (not (`self.isRedCP`)) (`self.isSelected`))
      (if (> ActionValue_Y 0.0)
        (`self.IncrementArray`)
        (`self.ChangeBeamColors` true)
        (else
          (`self.DecrementArray`)
          (`self.ChangeBeamColors` true))))))

(fn `ChangeBeamColors`
  (params (isSettingControlColor :type Boolean))
  (for _array_element (`self.ControlBeamsArray`)
    (`NiagaraComponent.SetVariableLinearColor` _array_element "User.Linear Color" (`self.NotControlColor`)))
  (if isSettingControlColor
    (`NiagaraComponent.SetVariableLinearColor` (`|GetArrayItem` (`self.ControlBeamsArray`) (`self.PosInArray`)) "User.Linear Color" (`self.ControlColor`))))

(fn `CreateObjectBeam`
  (params (InActor :type "Actor Object Reference"))
  (bind _returnvalue (`NiagaraFunctionLibrary.SpawnSystemAttached` "/Game/StopAndBreathe/Materials/ParticleSystems/P_ControlBeam2.P_ControlBeam2" (`self.Arrow`) "None" (0.0 0.0 0.0) (struct) "KeepRelativeOffset"))
  (`BlueprintMapLibrary.Map_Add` (`self.ActorNiagaraMap`) InActor _returnvalue)
  (`KismetArrayLibrary.Array_Add` (`self.ControlBeamsArray`) _returnvalue)
  (`FXSystemComponent.SetVectorParameter` _returnvalue "User.EndLoc" (`self.K2_GetActorLocation` InActor))
  (`ActorComponent.SetActive` _returnvalue false false)
  (`NiagaraComponent.SetVariableLinearColor` _returnvalue "User.Linear Color" (`self.NotControlColor`)))

(fn `DecrementArray`
  (bind _posinarray (`self.PosInArray`))
  (`/Engine/EditorBlueprintResources/StandardMacros.DecrementInt` (`self.PosInArray`)
    (:`  `
      (if (< (`self.PosInArray`) 0)
        (set `self.PosInArray` 0))
      (bind _output_get (set `self.ControlledObject` (`|GetArrayItem` (`self.AttachedObjects`) _posinarray)))
      (`KismetSystemLibrary.PrintString` (`KismetStringLibrary.Concat_StrStr` (`KismetStringLibrary.Conv_IntToString` _posinarray) (`KismetSystemLibrary.GetDisplayName` _output_get))))))

(fn `IncrementArray`
  (returns (ControlledObject :type "Actor Object Reference"))
  (bind _result (`/Engine/EditorBlueprintResources/StandardMacros.IncrementInt` (`self.PosInArray`))
    (:`  `
      (if (> (`self.PosInArray`) (- (`KismetArrayLibrary.Array_Length` (`self.AttachedObjects`)) 1))
        (set `self.PosInArray` (- (`KismetArrayLibrary.Array_Length` (`self.AttachedObjects`)) 1)))
      (bind _output_get (set `self.ControlledObject` (`|GetArrayItem` (`self.AttachedObjects`) (`self.PosInArray`))))
      (return _output_get))))

(fn `PlayFanAnim`
  (params (InState :type "/Game/StopAndBreathe/Blueprints/Interactables/ENUM_InteractableStates Enum" :default "NewEnumerator2"))
  (switch `/Game/StopAndBreathe/Blueprints/Interactables/ENUM_InteractableStates` InState
    (:`NewEnumerator2`
      (`SkeletalMeshComponent.Stop` (`self.SkeletalMesh`)))
    (:`NewEnumerator0`
      (`SkeletalMeshComponent.PlayAnimation` (`self.SkeletalMesh`) "/Game/StopAndBreathe/Assets/mechanic_assets/BreathingTerminal/Anim_FanSpin.Anim_FanSpin" true))
    (:`NewEnumerator1`
      (`SkeletalMeshComponent.PlayAnimation` (`self.SkeletalMesh`) "/Game/StopAndBreathe/Assets/mechanic_assets/BreathingTerminal/Anim_FanSpinReverse.Anim_FanSpinReverse" true))))

(fn `UserConstructionScript`
  (`parent.UserConstructionScript`)
  (if (`self.isRedCP`)
    (`PrimitiveComponent.SetMaterial` (`self.SkeletalMesh`) 0 "/Game/StopAndBreathe/Materials/AssetMaterials/BreathingTerminal/MAT_BreathingTerminalBase_Red.MAT_BreathingTerminalBase_Red")
    (`PrimitiveComponent.SetMaterial` (`self.SkeletalMesh`) 1 "/Game/StopAndBreathe/Materials/Development/Red_Mat.Red_Mat")
    (set `self.StartingMats` (`MeshComponent.GetMaterials` (`self.SkeletalMesh`)))
    (else
      (`PrimitiveComponent.SetMaterial` (`self.SkeletalMesh`) 0 "/Game/StopAndBreathe/Materials/AssetMaterials/BreathingTerminal/BreathingTerminalBase_Blue.BreathingTerminalBase_Blue")
      (`PrimitiveComponent.SetMaterial` (`self.SkeletalMesh`) 1 "/Game/StopAndBreathe/Materials/Development/Blue_Mat.Blue_Mat")
      (set `self.StartingMats` (`MeshComponent.GetMaterials` (`self.SkeletalMesh`))))))