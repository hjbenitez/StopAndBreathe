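; Breathing spot actor that flags the overlapping player character as inside a breathing trigger and shows an input prompt while they stay.
; It exposes an optional dialogue struct through getters, with its presence cached at BeginPlay.
; Once Done, which is not set here, Tick clears the player's trigger state, fades the spotlight over two seconds, then destroys the actor.
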(event `self.ReceiveBeginPlay`
  (`SceneComponent.SetHiddenInGame` (`self.Display Inputs`) true false)
  (set `self.hasDialogue?` (`KismetArrayLibrary.Array_IsNotEmpty` (`self.dialogueStruct`))))

(event `self.ReceiveActorBeginOverlap`
  (params (OtherActor :type "Actor Object Reference"))
  ;[1 0.2984 0.8739] Tell The Player BP That They Have Entered/Left A Breathing Spot
  (bind _output_get (set `self.player` OtherActor))
  (bind _asbp_third_person_character_particles (cast `/Game/ThirdPerson/Blueprints/BP_ThirdPersonCharacter_particles` _output_get))
  (if (not (`self.done`))
    (bind _output_get_2 (set `/Game/ThirdPerson/Blueprints/BP_ThirdPersonCharacter_particles.inBreathingTrigger` true _asbp_third_person_character_particles))
    (`SceneComponent.SetHiddenInGame` (`self.Display Inputs`) (not _output_get_2) false)))

(event `self.ReceiveActorEndOverlap`
  (params (OtherActor :type "Actor Object Reference"))
  ;[1 0.2984 0.8739] Tell The Player BP That They Have Entered/Left A Breathing Spot
  (bind _output_get (set `self.player` OtherActor))
  (bind _asbp_third_person_character_particles (cast `/Game/ThirdPerson/Blueprints/BP_ThirdPersonCharacter_particles` _output_get))
  (if (not (`self.done`))
    (bind _output_get_2 (set `/Game/ThirdPerson/Blueprints/BP_ThirdPersonCharacter_particles.inBreathingTrigger` false _asbp_third_person_character_particles))
    (`SceneComponent.SetHiddenInGame` (`self.Display Inputs`) (not _output_get_2) false)))

(event `self.ReceiveTick`
  (params (DeltaSeconds :type "Float (single-precision)"))
  ;[1 0.981 0.2425] Remove The Spot With a Smooth Transistion (Decrease The Light Intensity)
  (if (`self.done`)
    (bind _asbp_third_person_character_particles (cast `/Game/ThirdPerson/Blueprints/BP_ThirdPersonCharacter_particles` (`self.player`)))
    (set `/Game/ThirdPerson/Blueprints/BP_ThirdPersonCharacter_particles.inBreathingTrigger` false _asbp_third_person_character_particles)
    (set `/Game/ThirdPerson/Blueprints/BP_ThirdPersonCharacter_particles.recentBreathingTrigger` null _asbp_third_person_character_particles)
    (bind _output_get (set `self.lightTimer` (+ (`self.lightTimer`) (`GameplayStatics.GetWorldDeltaSeconds`))))
    (`LightComponent.SetIntensity` (`self.SpotLight`) (`KismetMathLibrary.Lerp` (`LightComponentBase.Intensity` (`self.SpotLight`)) 0.0 (/ _output_get 2.0)))
    (if (>= (`self.lightTimer`) 2.0)
      (`self.Remove Trigger`))))

(event `Remove Trigger`
  ;[1 0.07961 0.02985] Remove This Actor
  (`self.K2_DestroyActor`))

(fn `GetDialogue`
  (returns (dialogueStruct :type "Array of /Game/ThirdPerson/Blueprints/S_Dialogue Structure"))
  (return (`self.dialogueStruct`)))

(fn `HasDialogue`
  (returns (hasDialogue :type Boolean))
  (return (`self.hasDialogue?`)))

(fn `UserConstructionScript`)