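; Bumper is an actor that knocks pickeable boxes away when they overlap it, like a pinball bumper.
; On overlap with a BP_PickeableBox, it applies a large impulse to the box's static mesh, pointing away from the bumper's cylinder with random spread inside a cone.
; A leftover debug print fires on each hit, and other actors are ignored.
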(event `self.ReceiveActorBeginOverlap`
  (params (OtherActor :type "Actor Object Reference"))
  (bind _asbp_pickeable_box (cast `/Game/StopAndBreathe/Blueprints/Interactables/BP_PickeableBox` OtherActor))
  (`KismetSystemLibrary.PrintString` "Hello")
  (`PrimitiveComponent.AddImpulse` (`/Game/StopAndBreathe/Blueprints/Interactables/BP_BaseInteractable.StaticMesh` _asbp_pickeable_box) (* (`KismetMathLibrary.RandomUnitVectorInConeInDegrees` (`KismetMathLibrary.GetDirectionUnitVector` (`SceneComponent.K2_GetComponentLocation` (`self.Cylinder`)) (`self.K2_GetActorLocation` OtherActor)) 30.0) (250000.0 250000.0 250000.0)) "None" false))

(fn `UserConstructionScript`)